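; BP_Podium is an interactable podium that sets the player crab hero's score multiplier to its own value.
; Its collision overlap registers the podium as BP_CrabHero's overlapping interactable on entry, swaps in EmptyActor on exit, and calls SetInteractVisible both times.
; The Interact event copies ScoreMultiplier onto the hero and prints the new value.
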(event OnComponentBeginOverlap(collision)
  (params (OverlappedComponent :type Primitive%20Component%20Object%20Reference) (OtherActor :type Actor%20Object%20Reference) (OtherComp :type Primitive%20Component%20Object%20Reference) (OtherBodyIndex :type Integer) (bFromSweep :type Boolean) (SweepResult :type Hit%20Result%20Structure%20%28by%20ref%29))
  (bind _returnvalue (Game|Player|GetPlayerPawn 0))
  (if (== OtherActor _returnvalue)
    (bind _asbp_crab_hero (Utilities|Casting|CastToBP_CrabHero _returnvalue))
    (Variables|/Game/CrabGameFiles/Blueprints/ActorBlueprints/BP_CrabHero.BP_CrabHero_C|SetOverlappingInteractable _asbp_crab_hero self)
    (Default|SetInteractVisible _asbp_crab_hero)))

(event OnComponentEndOverlap(collision)
  (params (OverlappedComponent :type Primitive%20Component%20Object%20Reference) (OtherActor :type Actor%20Object%20Reference) (OtherComp :type Primitive%20Component%20Object%20Reference) (OtherBodyIndex :type Integer))
  (bind _returnvalue (Game|Player|GetPlayerPawn 0))
  (if (== OtherActor _returnvalue)
    (bind _asbp_crab_hero (Utilities|Casting|CastToBP_CrabHero _returnvalue))
    (Variables|/Game/CrabGameFiles/Blueprints/ActorBlueprints/BP_CrabHero.BP_CrabHero_C|SetOverlappingInteractable _asbp_crab_hero (Variables|Default|GetEmptyActor))
    (Default|SetInteractVisible _asbp_crab_hero)))

(event EventInteract
  (bind _asbp_crab_hero (Utilities|Casting|CastToBP_CrabHero (Game|Player|GetPlayerPawn 0)))
  (bind _output_get (Variables|/Game/CrabGameFiles/Blueprints/ActorBlueprints/BP_CrabHero.BP_CrabHero_C|SetScoreMultiplier _asbp_crab_hero (Variables|Default|GetScoreMultiplier)))
  (Development|PrintString (Utilities|String|Append "Score Multiplier:" (Utilities|String|ToString(Float) _output_get))))

(fn ConstructionScript)