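; Parent Blueprint for a buried food item that the crab player can dig up once for round score.
; On BeginPlay it picks a random mesh and binds its raise and lower movements to BP_Grid's grid square events.
; Box overlap registers it as BP_CrabHero's interactable and toggles the prompt.
; Interacting adds score and spins the mesh upward, then a timer fires an explosion and resets it to the unearthed height as a dug marker.
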(event OnComponentBeginOverlap(Boxcoll)
  (params (OverlappedComponent :type Primitive%20Component%20Object%20Reference) (OtherActor :type Actor%20Object%20Reference) (OtherComp :type Primitive%20Component%20Object%20Reference) (OtherBodyIndex :type Integer) (bFromSweep :type Boolean) (SweepResult :type Hit%20Result%20Structure%20%28by%20ref%29))
  (bind _returnvalue (Game|Player|GetPlayerPawn 0))
  (if (not (Variables|Default|GetHasBeenFound))
    (if (== OtherActor _returnvalue)
      (Variables|Default|SetIs%20Overlapping true)
      (bind _asbp_crab_hero (Utilities|Casting|CastToBP_CrabHero _returnvalue))
      (Default|SetInteractVisible _asbp_crab_hero)
      (if (Variables|Default|GetIs%20Overlapping)
        (Variables|/Game/CrabGameFiles/Blueprints/ActorBlueprints/BP_CrabHero.BP_CrabHero_C|SetOverlappingInteractable _asbp_crab_hero self)
        (else
          (Variables|/Game/CrabGameFiles/Blueprints/ActorBlueprints/BP_CrabHero.BP_CrabHero_C|SetOverlappingInteractable _asbp_crab_hero (Variables|Default|GetEmptyActor)))))))

(event OnComponentEndOverlap(Boxcoll)
  (params (OverlappedComponent :type Primitive%20Component%20Object%20Reference) (OtherActor :type Actor%20Object%20Reference) (OtherComp :type Primitive%20Component%20Object%20Reference) (OtherBodyIndex :type Integer))
  (if (not (Variables|Default|GetHasBeenFound))
    (if (== (Game|Player|GetPlayerPawn 0) OtherActor)
      (Variables|Default|SetIs%20Overlapping false)
      (Default|SetInteractInvisible (stale OnComponentBeginOverlap(Boxcoll) _asbp_crab_hero))
      (if (Variables|Default|GetIs%20Overlapping)
        (Variables|/Game/CrabGameFiles/Blueprints/ActorBlueprints/BP_CrabHero.BP_CrabHero_C|SetOverlappingInteractable (stale OnComponentBeginOverlap(Boxcoll) _asbp_crab_hero) self)
        (else
          (Variables|/Game/CrabGameFiles/Blueprints/ActorBlueprints/BP_CrabHero.BP_CrabHero_C|SetOverlappingInteractable (stale OnComponentBeginOverlap(Boxcoll) _asbp_crab_hero) (Variables|Default|GetEmptyActor)))))))

(event Custom|ResolveFoodSquare
  (Effects|SpawnEmitteratLocation "/Game/StarterContent/Particles/P_Explosion.P_Explosion" (Transformation|GetWorldLocation (Variables|Default|GetBaseMesh)) "0, 0, 0" "3.000000,3.000000,3.000000")
  ;[0.15 0.15 0.15 0.5] Place mesh back in the ground to let player know she has already dug this location
  (Variables|/Script/Engine.RotatingMovementComponent|SetRotationRate (Variables|Default|GetFoodRotatingMovement) "0, 0, 0")
  (Transformation|SetRelativeLocationAndRotation (Variables|Default|GetBaseMesh) (Math|Vector|MakeVector 0.0 0.0 (Variables|Default|GetUnearthedHeight)) "0, 0, 0" false false))

(event Custom|RaiseSelf
  ;[0.15 0.15 0.15 0.5] Called From Grid When Player Interacts with Podium to Reveal
  (Components|MoveComponentTo (Variables|Default|GetBaseMesh) (+ (Variables|/Script/Engine.SceneComponent|GetRelativeLocation (Variables|Default|GetBaseMesh)) (Variables|Default|GetRaiseHeight)) "0, 0, 0" false false 1.0 false))

(event Custom|LowerSelf
  ;[0.15 0.15 0.15 0.5] Called From Grid When Player Interacts with Podium to Reveal
  (Components|MoveComponentTo (Variables|Default|GetBaseMesh) (- (Variables|/Script/Engine.SceneComponent|GetRelativeLocation (Variables|Default|GetBaseMesh)) (Variables|Default|GetRaiseHeight)) "0, 0, 0" false false 1.0 false))

(event EventBeginPlay
  ;[0.15 0.15 0.15 0.5] Called From Grid When Player Interacts with Podium to Reveal
  (Components|StaticMesh|SetStaticMesh (Variables|Default|GetBaseMesh) (.OutItem (Utilities|Array|Random (Variables|Default|GetStaticMeshList))))
  (bind _returnvalue (Actor|GetActorOfClass "/Game/CrabGameFiles/Blueprints/ActorBlueprints/BP_Grid.BP_Grid_C"))
  (EventDispatchers|BindEventtoRaiseGridSquares _returnvalue (delegate Custom|RaiseSelf))
  (EventDispatchers|BindEventtoLowerGridSquares _returnvalue (delegate Custom|LowerSelf)))

(event EventInteract
  (if (not (Variables|Default|GetHasBeenFound))
    (if (Variables|Default|GetIs%20Overlapping)
      (Variables|Default|SetHasBeenFound true)
      (Utilities|FlowControl|Sequence
        (:then_0
          (Class|PlayerInterface|IncreaseRoundScore(Message) (Game|Player|GetPlayerPawn 0) (Variables|Default|GetScoreToAdd))
          (bind _returnvalue (AddComponent|AddRotatingMovementComponent))
          (Variables|Default|SetFoodRotatingMovement _returnvalue)
          (Components|MoveComponentTo (Variables|Default|GetBaseMesh) "0.000000,0.000000,250.000000" "0, 0, 0" false false 1.0 false)
          (Utilities|Time|SetTimerbyEvent (delegate Custom|ResolveFoodSquare) 0.5))
        (:then_1
          (bind _asbp_crab_hero (Utilities|Casting|CastToBP_CrabHero (Game|Player|GetPlayerPawn 0)))
          (Default|SetInteractInvisible _asbp_crab_hero))))))

(fn ConstructionScript)