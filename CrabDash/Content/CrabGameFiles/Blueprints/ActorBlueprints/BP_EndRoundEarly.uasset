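; BP_EndRoundEarly is an interactable actor that lets the crab hero end an ongoing round once all food is collected.
; Box overlap shows or hides the hero's interact prompt and sets or clears it as the overlapped interactable.
; On Interact, it counts food squares in BP_Grid and calls BP_RoundSystem's EndRoundEarly if RoundScore equals that count times the food's score value.
; Its EndRound and EndRoundEarly events reset the count.
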(event OnComponentBeginOverlap(Box)
  (params (OverlappedComponent :type Primitive%20Component%20Object%20Reference) (OtherActor :type Actor%20Object%20Reference) (OtherComp :type Primitive%20Component%20Object%20Reference) (OtherBodyIndex :type Integer) (bFromSweep :type Boolean) (SweepResult :type Hit%20Result%20Structure%20%28by%20ref%29))
  (bind _asbp_crab_hero (Utilities|Casting|CastToBP_CrabHero OtherActor))
  (bind _output_get (Variables|Default|SetAs%20BP%20Crab%20Hero _asbp_crab_hero))
  (Default|SetInteractVisible _output_get)
  (Variables|/Game/CrabGameFiles/Blueprints/ActorBlueprints/BP_CrabHero.BP_CrabHero_C|SetOverlappingInteractable _output_get self)
  (Variables|Default|SetIsOverlapping true))

(event OnComponentEndOverlap(Box)
  (params (OverlappedComponent :type Primitive%20Component%20Object%20Reference) (OtherActor :type Actor%20Object%20Reference) (OtherComp :type Primitive%20Component%20Object%20Reference) (OtherBodyIndex :type Integer))
  (bind _as_bp_crab_hero (Variables|Default|GetAs%20BP%20Crab%20Hero)
    (:then
      (Default|SetInteractInvisible _as_bp_crab_hero)
      (Variables|/Game/CrabGameFiles/Blueprints/ActorBlueprints/BP_CrabHero.BP_CrabHero_C|SetOverlappingInteractable _as_bp_crab_hero (Variables|Default|GetEmptyActor))
      (Variables|Default|SetIsOverlapping false))
    (:else)))

(event EventInteract
  ;[0.15 0.15 0.15 0.5] End Round Early Only If Round Ongoing (add and IF the player has collected all food squares)
  (bind _returnvalue (Actor|GetActorOfClass "/Game/CrabGameFiles/Blueprints/ActorBlueprints/BP_FoodParent.BP_FoodParent_C"))
  (Variables|Default|SetFoodScoreToAdd (Variables|/Game/CrabGameFiles/Blueprints/ActorBlueprints/BP_FoodParent.BP_FoodParent_C|GetScoreToAdd _returnvalue))
  (bind _asbp_crab_hero (Utilities|Casting|CastToBP_CrabHero (Game|Player|GetPlayerPawn 0)))
  (if (Variables|/Game/CrabGameFiles/Blueprints/ActorBlueprints/BP_CrabHero.BP_CrabHero_C|GetRoundOngoing? _asbp_crab_hero)
    (bind _returnvalue_2 (Actor|GetActorOfClass "/Game/CrabGameFiles/Blueprints/ActorBlueprints/BP_Grid.BP_Grid_C"))
    (for _array_element (Variables|/Game/CrabGameFiles/Blueprints/ActorBlueprints/BP_Grid.BP_Grid_C|GetGridArray _returnvalue_2)
      (if (== (.squaretype _array_element) 1)
        (Math|Integer|IncrementInt (Variables|Default|GetFoodSquaresInRound))))
    (if (== (Variables|/Game/CrabGameFiles/Blueprints/ActorBlueprints/BP_CrabHero.BP_CrabHero_C|GetRoundScore _asbp_crab_hero) (* (Variables|Default|GetFoodSquaresInRound) (Variables|Default|GetFoodScoreToAdd)))
      (bind _returnvalue_3 (Actor|GetActorOfClass "/Game/CrabGameFiles/Blueprints/ActorBlueprints/BP_RoundSystem.BP_RoundSystem_C"))
      (Default|EndRoundEarly _returnvalue_3))))

(event EventEndRound
  (Variables|Default|SetFoodSquaresInRound 0))

(event EventEndRoundEarly
  (Variables|Default|SetFoodSquaresInRound 0))

(fn ConstructionScript)