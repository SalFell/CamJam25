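; Prototype grid actor that builds a square grid of randomly typed squares and briefly reveals them once per round.
; BeginPlay fills GridArray with coordinates, then spawns one of three child actor components per cell and stores its type and reference.
; Reveal raises the squares and starts a timer; RevealEnd lowers them, then opens the platform boundary after a delay meant to let them sink fully.
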(event Custom|RevealEnd
  (bind _gridarray (Variables|Default|GetGridArray))
  (for (_array_element _array_index) _gridarray
    (Default|CallLowerGridSquares)
    (Utilities|Array|SetArrayElem _gridarray _array_index (Utilities|Struct|MakeGridSquareStructure (.row _array_element) (.collum _array_element) (.squaretype _array_element) (.squaretyperef _array_element)))
    ;[0.15 0.15 0.15 0.5] There's a better way to do this.... I need the boundary to open after the squares are fully underground
    (Utilities|FlowControl|Delay 1.0)
    (Default|CallOpenPlatformBoundary)))

(event EventBeginPlay
  ;[0.15 0.15 0.15 0.5] Replace with RoundRestart
  (Variables|Default|SetRoundRevealDone? false)
  (Utilities|FlowControl|Sequence
    (:then_0
      (for _index (range 0 (- (Variables|Default|GetGridRowCollumNumber) 1))
        (for _index_2 (range 0 (- (Variables|Default|GetGridRowCollumNumber) 1))
          (Utilities|Array|Add (Variables|Default|GetGridArray) (Utilities|Struct|MakeGridSquareStructure _index_2 _index 0 0)))))
    (:then_1
      (for (_array_element _array_index) (Variables|Default|GetGridArray)
        (bind _output_get (Variables|Default|SetSquareTypeSelector (Math|Random|RandomIntegerinRange 1 3)))
        (switch int _output_get
          (:1
            (bind _returnvalue (AddComponent|AddChildActorComponent false (Math|Transform|MakeTransform (Math|Vector|MakeVector (* (.row _array_element) (Variables|Default|GetSquareLocationOffset)) (* (.collum _array_element) (Variables|Default|GetSquareLocationOffset)) (Variables|Default|GetItemRevealHeight)) "0, 0, 0" "1.000000,1.000000,1.000000")))
            (Variables|Default|SetCurrentSquareTypeRef _returnvalue))
          (:2
            (bind _returnvalue_2 (AddComponent|AddChildActorComponent false (Math|Transform|MakeTransform (Math|Vector|MakeVector (* (.row _array_element) (Variables|Default|GetSquareLocationOffset)) (* (.collum _array_element) (Variables|Default|GetSquareLocationOffset)) (Variables|Default|GetItemRevealHeight)) "0, 0, 0" "1.000000,1.000000,1.000000")))
            (Variables|Default|SetCurrentSquareTypeRef _returnvalue_2))
          (:3
            (bind _returnvalue_3 (AddComponent|AddChildActorComponent false (Math|Transform|MakeTransform (Math|Vector|MakeVector (* (.row _array_element) (Variables|Default|GetSquareLocationOffset)) (* (.collum _array_element) (Variables|Default|GetSquareLocationOffset)) (Variables|Default|GetItemRevealHeight)) "0, 0, 0" "1.000000,1.000000,1.000000")))
            (Variables|Default|SetCurrentSquareTypeRef _returnvalue_3)))
        (Utilities|Array|SetArrayElem (Variables|Default|GetGridArray) _array_index (Utilities|Struct|MakeGridSquareStructure (.row _array_element) (.collum _array_element) _output_get (Variables|Default|GetCurrentSquareTypeRef)))))))

(event EventReveal
  (bind _gridarray (Variables|Default|GetGridArray))
  (Utilities|FlowControl|Sequence
    (:then_0
      (if (not (Variables|Default|GetRoundRevealDone?))
        (Variables|Default|SetRoundRevealDone? true)
        (for (_array_element _array_index) _gridarray
          (Default|CallRaiseGridSquares)
          (Utilities|Array|SetArrayElem _gridarray _array_index (Utilities|Struct|MakeGridSquareStructure (.row _array_element) (.collum _array_element) (.squaretype _array_element) (.squaretyperef _array_element)))
          (Utilities|Time|SetTimerbyEvent (delegate Custom|RevealEnd) (Variables|Default|GetRevealTimeSeconds)))))))

(fn ConstructionScript)