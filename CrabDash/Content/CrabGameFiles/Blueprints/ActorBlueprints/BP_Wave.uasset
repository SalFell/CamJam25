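; BP_Wave is the wave actor whose arrival at a limit actor ends the current round.
; BringinWave uses a DoOnce gate to raise the WaveOrigin component, then sweep it along Y with MoveComponentTo.
; When its Box overlaps the BP_WaveMaxDistance actor, it calls EndRound on BP_RoundSystem, snaps the wave back to the far negative Y side and resets the gate.
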(event OnComponentBeginOverlap(Box)
  (params (OverlappedComponent :type Primitive%20Component%20Object%20Reference) (OtherActor :type Actor%20Object%20Reference) (OtherComp :type Primitive%20Component%20Object%20Reference) (OtherBodyIndex :type Integer) (bFromSweep :type Boolean) (SweepResult :type Hit%20Result%20Structure%20%28by%20ref%29))
  (bind _waveorigin (Variables|Default|GetWaveOrigin))
  (if (== OtherActor (Variables|Default|GetWaveMaxDistanceRef))
    (bind _returnvalue (Actor|GetActorOfClass "/Game/CrabGameFiles/Blueprints/ActorBlueprints/BP_RoundSystem.BP_RoundSystem_C"))
    (Default|EndRound _returnvalue)
    (Components|MoveComponentTo (Variables|Default|GetWaveOrigin) "0.000000,-10850.000000,0.000000" "0, 0, 0" false false 0.1 false)
    (Utilities|FlowControl|DoOnce false) ; enters at Reset
  ))

(event EventBeginPlay
  (bind _returnvalue (Actor|GetActorOfClass "/Game/CrabGameFiles/Blueprints/ActorBlueprints/BP_WaveMaxDistance.BP_WaveMaxDistance_C"))
  (Variables|Default|SetWaveMaxDistanceRef _returnvalue)
  (Variables|Default|SetStartLocation (Transformation|GetActorLocation)))

(event EventBringinWave
  (bind _waveorigin (Variables|Default|GetWaveOrigin))
  (Utilities|FlowControl|DoOnce false
    (:Completed
      (Components|MoveComponentTo _waveorigin "0.000000,0.000000,450.000000" "0, 0, 0" false false 1.0 false)
      (Components|MoveComponentTo _waveorigin "0.000000,10850.000000,0.000000" "0, 0, 0" false false 5.0 false))))

(fn ConstructionScript)