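; BP_EmptySquare is an empty grid square that the crab hero can check once by interacting with it.
; It binds to BP_Grid's raise and lower events to slide its mesh up and down.
; Box overlaps toggle the hero's interact prompt and set its current interactable until the square is checked.
; Interacting marks it checked, hides the prompt, starts a quick mesh lift and sets a short timer to move it to its unearthed height.
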(event OnComponentBeginOverlap(Box)
  (params (OverlappedComponent :type Primitive%20Component%20Object%20Reference) (OtherActor :type Actor%20Object%20Reference) (OtherComp :type Primitive%20Component%20Object%20Reference) (OtherBodyIndex :type Integer) (bFromSweep :type Boolean) (SweepResult :type Hit%20Result%20Structure%20%28by%20ref%29))
  (if (not (Variables|Default|GetHasBeenChecked))
    (bind _asbp_crab_hero (Utilities|Casting|CastToBP_CrabHero OtherActor))
    (Default|SetInteractVisible _asbp_crab_hero)
    (Variables|/Game/CrabGameFiles/Blueprints/ActorBlueprints/BP_CrabHero.BP_CrabHero_C|SetOverlappingInteractable _asbp_crab_hero self)
    (Variables|Default|SetIsOverlapping true)))

(event OnComponentEndOverlap(Box)
  (params (OverlappedComponent :type Primitive%20Component%20Object%20Reference) (OtherActor :type Actor%20Object%20Reference) (OtherComp :type Primitive%20Component%20Object%20Reference) (OtherBodyIndex :type Integer))
  (if (not (Variables|Default|GetHasBeenChecked))
    (bind _asbp_crab_hero (Utilities|Casting|CastToBP_CrabHero OtherActor))
    (Default|SetInteractInvisible _asbp_crab_hero)
    (Variables|/Game/CrabGameFiles/Blueprints/ActorBlueprints/BP_CrabHero.BP_CrabHero_C|SetOverlappingInteractable _asbp_crab_hero (Variables|Default|GetEmptyActor))
    (Variables|Default|SetIsOverlapping false)))

(event Custom|LowerEmptySquare
  (Components|MoveComponentTo (Variables|Default|GetBaseMesh) (Math|Vector|MakeVector 0.0 0.0 (Variables|Default|GetUnearthedHeight)) "0, 0, 0" false false 0.5 false))

(event Custom|RaiseSelf
  ;[0.15 0.15 0.15 0.5] Called From Grid When Player Interacts with Podium to Reveal
  (Components|MoveComponentTo (Variables|Default|GetBaseMesh) (+ (Variables|/Script/Engine.SceneComponent|GetRelativeLocation (Variables|Default|GetBaseMesh)) "0.000000,0.000000,200.000000") "0, 0, 0" false false 1.0 false))

(event Custom|LowerSelf
  ;[0.15 0.15 0.15 0.5] Called From Grid When Player Interacts with Podium to Reveal
  (Components|MoveComponentTo (Variables|Default|GetBaseMesh) (- (Variables|/Script/Engine.SceneComponent|GetRelativeLocation (Variables|Default|GetBaseMesh)) "0.000000,0.000000,200.000000") "0, 0, 0" false false 1.0 false))

(event EventBeginPlay
  ;[0.15 0.15 0.15 0.5] Called From Grid When Player Interacts with Podium to Reveal
  (bind _returnvalue (Actor|GetActorOfClass "/Game/CrabGameFiles/Blueprints/ActorBlueprints/BP_Grid.BP_Grid_C"))
  (EventDispatchers|BindEventtoRaiseGridSquares _returnvalue (delegate Custom|RaiseSelf))
  (EventDispatchers|BindEventtoLowerGridSquares _returnvalue (delegate Custom|LowerSelf)))

(event EventInteract
  (if (not (Variables|Default|GetHasBeenChecked))
    (if (Variables|Default|GetIsOverlapping)
      (Variables|Default|SetHasBeenChecked true)
      (bind _asbp_crab_hero (Utilities|Casting|CastToBP_CrabHero (Game|Player|GetPlayerPawn 0)))
      (Default|SetInteractInvisible _asbp_crab_hero)
      (Components|MoveComponentTo (Variables|Default|GetBaseMesh) "0.000000,0.000000,250.000000" "0, 0, 0" false false 0.3 false)
      (Utilities|Time|SetTimerbyEvent (delegate Custom|LowerEmptySquare) 0.1))))

(fn ConstructionScript)