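; BP_HazardSquare is a one-time grid hazard that stuns the crab player who interacts with it.
; Its box overlap registers it as the hero's interactable and toggles the prompt.
; Interacting disables input and pops the crab mesh up, then timers lower it and restore input unless underwater.
; It also binds to BP_Grid's raise and lower events, sliding the mesh by RaiseHeight for reveals.
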(event OnComponentBeginOverlap(Box)
  (params (OverlappedComponent :type Primitive%20Component%20Object%20Reference) (OtherActor :type Actor%20Object%20Reference) (OtherComp :type Primitive%20Component%20Object%20Reference) (OtherBodyIndex :type Integer) (bFromSweep :type Boolean) (SweepResult :type Hit%20Result%20Structure%20%28by%20ref%29))
  ;[0.15 0.15 0.15 0.5] Check if player is overlapping with this object
  (if (not (Variables|Default|GetHasActivated))
    (if (Class|GameplayStatics|ObjectIsA OtherActor "/Game/CrabGameFiles/Blueprints/ActorBlueprints/BP_CrabHero.BP_CrabHero_C")
      (Variables|Default|SetIsOverlapping true)
      (bind _output_get (Variables|Default|SetPlayerCrab OtherActor))
      (bind _asbp_crab_hero (Utilities|Casting|CastToBP_CrabHero _output_get))
      (Default|SetInteractVisible _asbp_crab_hero)
      (if true
        (Variables|/Game/CrabGameFiles/Blueprints/ActorBlueprints/BP_CrabHero.BP_CrabHero_C|SetOverlappingInteractable _asbp_crab_hero self)))))

(event OnComponentBeginOverlap(BaseSquare)
  (params (OverlappedComponent :type Primitive%20Component%20Object%20Reference) (OtherActor :type Actor%20Object%20Reference) (OtherComp :type Primitive%20Component%20Object%20Reference) (OtherBodyIndex :type Integer) (bFromSweep :type Boolean) (SweepResult :type Hit%20Result%20Structure%20%28by%20ref%29)))

(event OnComponentEndOverlap(Box)
  (params (OverlappedComponent :type Primitive%20Component%20Object%20Reference) (OtherActor :type Actor%20Object%20Reference) (OtherComp :type Primitive%20Component%20Object%20Reference) (OtherBodyIndex :type Integer))
  (if (Class|GameplayStatics|ObjectIsA OtherActor "/Game/CrabGameFiles/Blueprints/ActorBlueprints/BP_CrabHero.BP_CrabHero_C")
    (Variables|Default|SetIsOverlapping false)
    (bind _asbp_crab_hero (Utilities|Casting|CastToBP_CrabHero OtherActor))
    (Default|SetInteractInvisible _asbp_crab_hero)
    (if true
      (Variables|/Game/CrabGameFiles/Blueprints/ActorBlueprints/BP_CrabHero.BP_CrabHero_C|SetOverlappingInteractable _asbp_crab_hero (Variables|Default|GetEmptyActor)))))

(event Custom|RaiseSelf
  ;[0.15 0.15 0.15 0.5] Called From Grid When Player Interacts with Podium to Reveal
  (Components|MoveComponentTo (Variables|Default|GetBaseSquare) (+ (Variables|/Script/Engine.SceneComponent|GetRelativeLocation (Variables|Default|GetBaseSquare)) (Variables|Default|GetRaiseHeight)) "0, 0, 0" false false 1.0 false))

(event Custom|LowerSquare
  (Components|MoveComponentTo (Variables|Default|GetBaseSquare) (Math|Vector|MakeVector 0.0 0.0 (Variables|Default|GetUnearthedHeight)) "0, 0, 0" false false 2.0 false))

(event Custom|LowerSelf
  ;[0.15 0.15 0.15 0.5] Called From Grid When Player Interacts with Podium to Reveal
  (Components|MoveComponentTo (Variables|Default|GetBaseSquare) (- (Variables|/Script/Engine.SceneComponent|GetRelativeLocation (Variables|Default|GetBaseSquare)) (Variables|Default|GetRaiseHeight)) "0, 0, 0" false false 1.0 false))

(event Custom|EnableInputEvent
  ;[0.15 0.15 0.15 0.5] Stun player
  (if (Variables|/Game/CrabGameFiles/Blueprints/ActorBlueprints/BP_CrabHero.BP_CrabHero_C|GetIsUnderwater (stale EventInteract _asbp_crab_hero))
    _
    (else
      (Input|EnableInput (Variables|Default|GetPlayerCrab) (Game|GetPlayerController 0))))
  (Variables|Default|SetHasActivated true))

(event EventBeginPlay
  ;[0.15 0.15 0.15 0.5] Called From Grid When Player Interacts with Podium to Reveal
  (Components|StaticMesh|SetStaticMesh (Variables|Default|GetBaseSquare) "/Game/CrabGameFiles/Meshes/HazardCrab/CAMJAM_Crab.CAMJAM_Crab")
  (bind _returnvalue (Actor|GetActorOfClass "/Game/CrabGameFiles/Blueprints/ActorBlueprints/BP_Grid.BP_Grid_C"))
  (EventDispatchers|BindEventtoRaiseGridSquares _returnvalue (delegate Custom|RaiseSelf))
  (EventDispatchers|BindEventtoLowerGridSquares _returnvalue (delegate Custom|LowerSelf)))

(event EventInteract
  (bind _playercrab (Variables|Default|GetPlayerCrab))
  (if (not (Variables|Default|GetHasActivated))
    (if (Variables|Default|GetIsOverlapping)
      (Utilities|FlowControl|Sequence
        (:then_0
          ;[0.15 0.15 0.15 0.5] Stun player
          (bind _asbp_crab_hero (Utilities|Casting|CastToBP_CrabHero _playercrab))
          (Default|SetInteractInvisible _asbp_crab_hero)
          (Input|DisableInput _playercrab (Game|GetPlayerController 0))
          (Utilities|Time|SetTimerbyEvent (delegate Custom|EnableInputEvent) (Variables|Default|GetStunDuration)))
        (:then_1
          (Components|MoveComponentTo (Variables|Default|GetBaseSquare) "0.000000,0.000000,250.000000" "0, 0, 0" false false 1.0 false)
          (Utilities|Time|SetTimerbyEvent (delegate Custom|LowerSquare) 2.0))))))

(fn ConstructionScript)