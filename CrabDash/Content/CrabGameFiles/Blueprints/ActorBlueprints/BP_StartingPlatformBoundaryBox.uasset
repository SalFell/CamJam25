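; Boundary actor for the starting platform that controls when the area is blocked and detects crab heroes crossing its exit volume.
; On BeginPlay it binds to the grid's open-boundary event, which disables the Box collision, and to BP_EndRoundEarly's end-round event to restore it.
; Overlapping ExitingBox messages a BP_CrabHero to start its timer and marks it as no longer safe.
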(event OnComponentBeginOverlap(ExitingBox)
  (params (OverlappedComponent :type Primitive%20Component%20Object%20Reference) (OtherActor :type Actor%20Object%20Reference) (OtherComp :type Primitive%20Component%20Object%20Reference) (OtherBodyIndex :type Integer) (bFromSweep :type Boolean) (SweepResult :type Hit%20Result%20Structure%20%28by%20ref%29))
  (if (Class|GameplayStatics|ObjectIsA OtherActor "/Game/CrabGameFiles/Blueprints/ActorBlueprints/BP_CrabHero.BP_CrabHero_C")
    (Class|PlayerInterface|StartTimer(Message) OtherActor)
    (Class|PlayerInterface|SetIsSafe(Message) OtherActor false)))

(event Custom|OpenBoundary
  (Collision|SetCollisionEnabled (Variables|Default|GetBox) "NoCollision"))

(event Custom|EndRound
  (params (IsOverlapping :type Boolean))
  (Collision|SetCollisionEnabled (Variables|Default|GetBox) "QueryAndPhysics"))

(event EventBeginPlay
  (EventDispatchers|BindEventtoOpenPlatformBoundary (Variables|Default|GetGridRef) (delegate Custom|OpenBoundary))
  (bind _returnvalue (Actor|GetActorOfClass "/Game/CrabGameFiles/Blueprints/ActorBlueprints/BP_EndRoundEarly.BP_EndRoundEarly_C"))
  (bind _output_get (Variables|Default|SetEndRoundEarlyRef _returnvalue))
  (EventDispatchers|BindEventtoEndRound _output_get (EventDispatchers|CreateEvent :!event Custom|EndRound)))

(fn ConstructionScript)