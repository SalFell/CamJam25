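; Music manager for the crab game that switches between main menu, in-game and fail-state themes.
; Each play event fades out the other two tracks, then restarts its cached audio component or spawns one that persists across level transitions.
; On first play, the game theme runs its intro for a fixed 8-second delay before starting the loop; the audio-finished binding meant for this handoff is disconnected.
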(event Custom|Play%20Game%20Track%20%28inGame%29
  ;[0.07731 0.1192 0.15 0.5] Music Manager
  (Development|PrintString "Play Game Track Music Instnacxe" true true "(R=1.000000,G=0.491287,B=0.851714,A=1.000000)" 4.0)
  (CallFunction|StopMainTrack(Menu))
  (CallFunction|StopFailState(inGame))
  (Utilities|IsValid (Variables|Default|GetGame%20Music%20Track)
    (:Is%20Valid
      (if (not (Audio|Components|Audio|IsPlaying (Variables|Default|GetGame%20Music%20Track)))
        (Audio|Components|Audio|Play (Variables|Default|GetGame%20Music%20Track) 0.0)))
    (:Is%20Not%20Valid
      (bind _returnvalue (Audio|SpawnSound2D "/Game/CrabGameFiles/Audio/Music/CrabDash_Music_InGameTheme_Intro_.CrabDash_Music_InGameTheme_Intro_" 1.0 1.0 0.0 "/Game/CrabGameFiles/Blueprints/SC_MusicConcurrency.SC_MusicConcurrency" true false))
      (Utilities|FlowControl|Delay 8.0)
      (Audio|Components|Audio|FadeOut _returnvalue 0.5 0.0 "Linear" :!class /Script/Engine.AudioComponent)
      (bind _returnvalue_2 (Audio|SpawnSound2D "/Game/CrabGameFiles/Audio/Music/CrabDash_Music_InGameTheme_MainLoop_.CrabDash_Music_InGameTheme_MainLoop_" 1.0 1.0 0.0 "/Game/CrabGameFiles/Blueprints/SC_MusicConcurrency.SC_MusicConcurrency" true false))
      (Variables|Default|SetGame%20Music%20Track _returnvalue_2))))

(event Custom|Play%20Main%20Track%20%28Menu%29
  ;[0.07731 0.1192 0.15 0.5] Music Manager
  (Development|PrintString "Music Instance main track playing" true true "(R=0.021752,G=1.000000,B=0.000000,A=1.000000)" 4.0)
  (CallFunction|StopFailState(inGame))
  (CallFunction|StopGameTrack(inGame))
  (Utilities|IsValid (Variables|Default|GetMain%20Music%20Track)
    (:Is%20Valid
      (if (not (Audio|Components|Audio|IsPlaying (Variables|Default|GetMain%20Music%20Track)))
        (Audio|Components|Audio|Play (Variables|Default|GetMain%20Music%20Track) 0.0)))
    (:Is%20Not%20Valid
      (bind _returnvalue (Audio|SpawnSound2D "/Game/CrabGameFiles/Audio/Music/CrabDash_Music_MainTheme.CrabDash_Music_MainTheme" 1.0 1.0 0.0 "/Game/CrabGameFiles/Blueprints/SC_MusicConcurrency.SC_MusicConcurrency" true false))
      (Variables|Default|SetMain%20Music%20Track _returnvalue))))

(event Custom|PlayLoop
  ;[0.15 0.15 0.15 0.5] Proper way isn't working?
  (Development|PrintString "Started Game loop audio" true true "(R=1.000000,G=0.683656,B=0.360413,A=1.000000)" 5.0))

(event Custom|Stop%20Game%20Track%20%28inGame%29
  (bind _game_music_track (Variables|Default|GetGame%20Music%20Track))
  ;[0.07731 0.1192 0.15 0.5] Music Manager
  (Utilities|IsValid _game_music_track
    (:Is%20Valid
      (if (Audio|Components|Audio|IsPlaying _game_music_track)
        (Audio|Components|Audio|FadeOut _game_music_track 0.5 0.0 "Linear" :!class /Script/Engine.AudioComponent)))))

(event Custom|Play%20Fail%20State%20%28inGame%29
  ;[0.07731 0.1192 0.15 0.5] Music Manager
  (Development|PrintString "Fail State Music Started" true true "(R=1.000000,G=0.009947,B=0.000000,A=1.000000)")
  (CallFunction|StopMainTrack(Menu))
  (CallFunction|StopGameTrack(inGame))
  (Utilities|IsValid (Variables|Default|GetFail%20Music%20Track)
    (:Is%20Valid
      (if (not (Audio|Components|Audio|IsPlaying (Variables|Default|GetFail%20Music%20Track)))
        (Audio|Components|Audio|Play (Variables|Default|GetFail%20Music%20Track) 0.0)))
    (:Is%20Not%20Valid
      (bind _returnvalue (Audio|SpawnSound2D "/Game/CrabGameFiles/Audio/Music/CrabDash_Music_FailStateTheme_Loop_.CrabDash_Music_FailStateTheme_Loop_" 1.0 1.0 0.0 "/Game/CrabGameFiles/Blueprints/SC_MusicConcurrency.SC_MusicConcurrency" true false))
      (Variables|Default|SetFail%20Music%20Track _returnvalue))))

(event Custom|Stop%20Fail%20State%20%28inGame%29
  (bind _fail_music_track (Variables|Default|GetFail%20Music%20Track))
  ;[0.07731 0.1192 0.15 0.5] Music Manager
  (Utilities|IsValid _fail_music_track
    (:Is%20Valid
      (if (Audio|Components|Audio|IsPlaying _fail_music_track)
        (Audio|Components|Audio|FadeOut _fail_music_track 0.5 0.0 "Linear" :!class /Script/Engine.AudioComponent)))))

(event Custom|Stop%20Main%20Track%20%28Menu%29
  (bind _main_music_track (Variables|Default|GetMain%20Music%20Track))
  ;[0.07731 0.1192 0.15 0.5] Music Manager
  (Utilities|IsValid _main_music_track
    (:Is%20Valid
      (if (Audio|Components|Audio|IsPlaying _main_music_track)
        (Audio|Components|Audio|FadeOut _main_music_track 0.5 0.0 "Linear" :!class /Script/Engine.AudioComponent)))))