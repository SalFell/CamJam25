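; Prototype grid board that spawns square meshes, each with one of three randomly chosen child actors, hidden at start.
; BeginPlay stores each cell's position, type, visibility and actor reference in GridArray.
; Reveal shows all items and starts a timer to RevealEnd, which clears the visible flag but still sets components visible.
; Two unfinished random-walk path generators, PathCreation and PathCreation2, are unused; random type selection stands in for them.
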(event Custom|RevealEnd
  (bind _gridarray (Variables|Default|GetGridArray))
  (for (_array_element _array_index) _gridarray
    (Rendering|SetVisibility (.squaretyperef _array_element) true false)
    (Utilities|Array|SetArrayElem _gridarray _array_index (Utilities|Struct|MakeGridSquareStructure (.row _array_element) (.collum _array_element) (.squaretype _array_element) false (.squaretyperef _array_element)))))

(event EventBeginPlay
  ;[0.15 0.15 0.15 0.5] Replace with RoundRestart
  (Utilities|FlowControl|Sequence
    (:then_0
      (for _index (range 0 (- (Variables|Default|GetGridRowCollumNumber) 1))
        (for _index_2 (range 0 (- (Variables|Default|GetGridRowCollumNumber) 1))
          (Utilities|Array|Add (Variables|Default|GetGridArray) (Utilities|Struct|MakeGridSquareStructure _index_2 _index 0 false 0)))))
    (:then_1)
    (:then_2
      (for (_array_element _array_index) (Variables|Default|GetGridArray)
        (AddComponent|AddStaticMeshComponent false (Math|Transform|MakeTransform (Math|Vector|MakeVector (* (.row _array_element) (Variables|Default|GetSquareLocationOffset)) (* (.collum _array_element) (Variables|Default|GetSquareLocationOffset)) 0.0) "0, 0, 0" "1.000000,1.000000,1.000000"))
        (bind _output_get (Variables|Default|SetSquareTypeSelector (Math|Random|RandomIntegerinRange 1 3)))
        (switch int _output_get
          (:1
            (bind _returnvalue (AddComponent|AddChildActorComponent false (Math|Transform|MakeTransform (Math|Vector|MakeVector (* (.row _array_element) (Variables|Default|GetSquareLocationOffset)) (* (.collum _array_element) (Variables|Default|GetSquareLocationOffset)) (Variables|Default|GetItemRevealHeight)) "0, 0, 0" "1.000000,1.000000,1.000000")))
            (Variables|Default|SetCurrentSquareTypeRef _returnvalue))
          (:2
            (bind _returnvalue_2 (AddComponent|AddChildActorComponent false (Math|Transform|MakeTransform (Math|Vector|MakeVector (* (.row _array_element) (Variables|Default|GetSquareLocationOffset)) (* (.collum _array_element) (Variables|Default|GetSquareLocationOffset)) (Variables|Default|GetItemRevealHeight)) "0, 0, 0" "1.000000,1.000000,1.000000")))
            (Variables|Default|SetCurrentSquareTypeRef _returnvalue_2))
          (:3
            (bind _returnvalue_3 (AddComponent|AddChildActorComponent false (Math|Transform|MakeTransform (Math|Vector|MakeVector (* (.row _array_element) (Variables|Default|GetSquareLocationOffset)) (* (.collum _array_element) (Variables|Default|GetSquareLocationOffset)) (Variables|Default|GetItemRevealHeight)) "0, 0, 0" "1.000000,1.000000,1.000000")))
            (Variables|Default|SetCurrentSquareTypeRef _returnvalue_3)))
        (Rendering|SetVisibility (Variables|Default|GetCurrentSquareTypeRef) false false)
        (Utilities|Array|SetArrayElem (Variables|Default|GetGridArray) _array_index (Utilities|Struct|MakeGridSquareStructure (.row _array_element) (.collum _array_element) _output_get false (Variables|Default|GetCurrentSquareTypeRef)))))))

(event EventReveal
  (bind _gridarray (Variables|Default|GetGridArray))
  (for (_array_element _array_index) _gridarray
    (Rendering|SetVisibility (.squaretyperef _array_element) true false)
    (Utilities|Array|SetArrayElem _gridarray _array_index (Utilities|Struct|MakeGridSquareStructure (.row _array_element) (.collum _array_element) (.squaretype _array_element) true (.squaretyperef _array_element)))
    (Utilities|Time|SetTimerbyEvent (delegate Custom|RevealEnd) (Variables|Default|GetRevealTimeSeconds))))

(fn ConstructionScript)

(fn PathCreation
  (bind _returnvalue (Math|Random|RandomIntegerinRange 0 4))
  (bind _gridarray (Variables|Default|GetGridArray))
  (bind _gridarray_2 (Variables|Default|GetGridArray))
  (bind _gridarray_3 (Variables|Default|GetGridArray))
  (bind _gridarray_4 (Variables|Default|GetGridArray))
  (bind _gridarray_5 (Variables|Default|GetGridArray))
  (bind _gridarray_6 (Variables|Default|GetGridArray))
  (bind _tempgridarray (Variables|Default|GetTempGridArray))
  (bind _output (Utilities|Array|Get(acopy) _gridarray_2 _returnvalue))
  ;[0.15 0.15 0.15 0.5 41] I give up on this version
  (Utilities|FlowControl|Sequence
    (:then_0
      (bind _output_get (Variables|Default|SetTempSquareType (Math|Random|RandomIntegerinRange 1 2)))
      (Utilities|Array|SetArrayElem _gridarray_2 _returnvalue (Utilities|Struct|MakeGridSquareStructure (.row _output) (.collum _output) _output_get (.visible? _output) (.squaretyperef _output)))
      (Variables|Default|SetNextPathSquareIndex _returnvalue))
    (:then_1
      (Utilities|FlowControl|ForLoopwithBreak 0 10 :!label _label
        (:LoopBody
          (Utilities|FlowControl|Sequence
            (:then_0
              (if (and (Utilities|Array|IsValidIndex _gridarray (Utilities|Array|FindItem _gridarray (Utilities|Struct|MakeGridSquareStructure (.row (Utilities|Array|Get(acopy) _gridarray (Variables|Default|GetNextPathSquareIndex))) (+ (.collum (Utilities|Array|Get(acopy) _gridarray (Variables|Default|GetNextPathSquareIndex))) 1) (.squaretype (Utilities|Array|Get(acopy) _gridarray (Variables|Default|GetNextPathSquareIndex))) (.visible? (Utilities|Array|Get(acopy) _gridarray (Variables|Default|GetNextPathSquareIndex))) (.squaretyperef (Utilities|Array|Get(acopy) _gridarray (Variables|Default|GetNextPathSquareIndex)))))) (== (.squaretype (Utilities|Array|Get(acopy) _gridarray (Utilities|Array|FindItem _gridarray (Utilities|Struct|MakeGridSquareStructure (.row (Utilities|Array|Get(acopy) _gridarray (Variables|Default|GetNextPathSquareIndex))) (+ (.collum (Utilities|Array|Get(acopy) _gridarray (Variables|Default|GetNextPathSquareIndex))) 1) (.squaretype (Utilities|Array|Get(acopy) _gridarray (Variables|Default|GetNextPathSquareIndex))) (.visible? (Utilities|Array|Get(acopy) _gridarray (Variables|Default|GetNextPathSquareIndex))) (.squaretyperef (Utilities|Array|Get(acopy) _gridarray (Variables|Default|GetNextPathSquareIndex))))))) 0))
                (Utilities|Array|Add (Variables|Default|GetTempGridArray) (Utilities|Struct|MakeGridSquareStructure (.row (Utilities|Array|Get(acopy) _gridarray (Utilities|Array|FindItem _gridarray (Utilities|Struct|MakeGridSquareStructure (.row (Utilities|Array|Get(acopy) _gridarray (Variables|Default|GetNextPathSquareIndex))) (+ (.collum (Utilities|Array|Get(acopy) _gridarray (Variables|Default|GetNextPathSquareIndex))) 1) (.squaretype (Utilities|Array|Get(acopy) _gridarray (Variables|Default|GetNextPathSquareIndex))) (.visible? (Utilities|Array|Get(acopy) _gridarray (Variables|Default|GetNextPathSquareIndex))) (.squaretyperef (Utilities|Array|Get(acopy) _gridarray (Variables|Default|GetNextPathSquareIndex))))))) (.collum (Utilities|Array|Get(acopy) _gridarray (Utilities|Array|FindItem _gridarray (Utilities|Struct|MakeGridSquareStructure (.row (Utilities|Array|Get(acopy) _gridarray (Variables|Default|GetNextPathSquareIndex))) (+ (.collum (Utilities|Array|Get(acopy) _gridarray (Variables|Default|GetNextPathSquareIndex))) 1) (.squaretype (Utilities|Array|Get(acopy) _gridarray (Variables|Default|GetNextPathSquareIndex))) (.visible? (Utilities|Array|Get(acopy) _gridarray (Variables|Default|GetNextPathSquareIndex))) (.squaretyperef (Utilities|Array|Get(acopy) _gridarray (Variables|Default|GetNextPathSquareIndex))))))) (.squaretype (Utilities|Array|Get(acopy) _gridarray (Utilities|Array|FindItem _gridarray (Utilities|Struct|MakeGridSquareStructure (.row (Utilities|Array|Get(acopy) _gridarray (Variables|Default|GetNextPathSquareIndex))) (+ (.collum (Utilities|Array|Get(acopy) _gridarray (Variables|Default|GetNextPathSquareIndex))) 1) (.squaretype (Utilities|Array|Get(acopy) _gridarray (Variables|Default|GetNextPathSquareIndex))) (.visible? (Utilities|Array|Get(acopy) _gridarray (Variables|Default|GetNextPathSquareIndex))) (.squaretyperef (Utilities|Array|Get(acopy) _gridarray (Variables|Default|GetNextPathSquareIndex))))))) (.visible? (Utilities|Array|Get(acopy) _gridarray (Utilities|Array|FindItem _gridarray (Utilities|Struct|MakeGridSquareStructure (.row (Utilities|Array|Get(acopy) _gridarray (Variables|Default|GetNextPathSquareIndex))) (+ (.collum (Utilities|Array|Get(acopy) _gridarray (Variables|Default|GetNextPathSquareIndex))) 1) (.squaretype (Utilities|Array|Get(acopy) _gridarray (Variables|Default|GetNextPathSquareIndex))) (.visible? (Utilities|Array|Get(acopy) _gridarray (Variables|Default|GetNextPathSquareIndex))) (.squaretyperef (Utilities|Array|Get(acopy) _gridarray (Variables|Default|GetNextPathSquareIndex))))))) (.squaretyperef (Utilities|Array|Get(acopy) _gridarray (Utilities|Array|FindItem _gridarray (Utilities|Struct|MakeGridSquareStructure (.row (Utilities|Array|Get(acopy) _gridarray (Variables|Default|GetNextPathSquareIndex))) (+ (.collum (Utilities|Array|Get(acopy) _gridarray (Variables|Default|GetNextPathSquareIndex))) 1) (.squaretype (Utilities|Array|Get(acopy) _gridarray (Variables|Default|GetNextPathSquareIndex))) (.visible? (Utilities|Array|Get(acopy) _gridarray (Variables|Default|GetNextPathSquareIndex))) (.squaretyperef (Utilities|Array|Get(acopy) _gridarray (Variables|Default|GetNextPathSquareIndex)))))))))))
            (:then_1
              (if (and (Utilities|Array|IsValidIndex _gridarray_5 (Utilities|Array|FindItem _gridarray_5 (Utilities|Struct|MakeGridSquareStructure (+ (.row (Utilities|Array|Get(acopy) _gridarray_5 (Variables|Default|GetNextPathSquareIndex))) 1) (.collum (Utilities|Array|Get(acopy) _gridarray_5 (Variables|Default|GetNextPathSquareIndex))) (.squaretype (Utilities|Array|Get(acopy) _gridarray_5 (Variables|Default|GetNextPathSquareIndex))) (.visible? (Utilities|Array|Get(acopy) _gridarray_5 (Variables|Default|GetNextPathSquareIndex))) (.squaretyperef (Utilities|Array|Get(acopy) _gridarray_5 (Variables|Default|GetNextPathSquareIndex)))))) (== (.squaretype (Utilities|Array|Get(acopy) _gridarray_5 (Utilities|Array|FindItem _gridarray_5 (Utilities|Struct|MakeGridSquareStructure (+ (.row (Utilities|Array|Get(acopy) _gridarray_5 (Variables|Default|GetNextPathSquareIndex))) 1) (.collum (Utilities|Array|Get(acopy) _gridarray_5 (Variables|Default|GetNextPathSquareIndex))) (.squaretype (Utilities|Array|Get(acopy) _gridarray_5 (Variables|Default|GetNextPathSquareIndex))) (.visible? (Utilities|Array|Get(acopy) _gridarray_5 (Variables|Default|GetNextPathSquareIndex))) (.squaretyperef (Utilities|Array|Get(acopy) _gridarray_5 (Variables|Default|GetNextPathSquareIndex))))))) 0))
                (Utilities|Array|Add (Variables|Default|GetTempGridArray) (Utilities|Struct|MakeGridSquareStructure (.row (Utilities|Array|Get(acopy) _gridarray_5 (Utilities|Array|FindItem _gridarray_5 (Utilities|Struct|MakeGridSquareStructure (+ (.row (Utilities|Array|Get(acopy) _gridarray_5 (Variables|Default|GetNextPathSquareIndex))) 1) (.collum (Utilities|Array|Get(acopy) _gridarray_5 (Variables|Default|GetNextPathSquareIndex))) (.squaretype (Utilities|Array|Get(acopy) _gridarray_5 (Variables|Default|GetNextPathSquareIndex))) (.visible? (Utilities|Array|Get(acopy) _gridarray_5 (Variables|Default|GetNextPathSquareIndex))) (.squaretyperef (Utilities|Array|Get(acopy) _gridarray_5 (Variables|Default|GetNextPathSquareIndex))))))) (.collum (Utilities|Array|Get(acopy) _gridarray_5 (Utilities|Array|FindItem _gridarray_5 (Utilities|Struct|MakeGridSquareStructure (+ (.row (Utilities|Array|Get(acopy) _gridarray_5 (Variables|Default|GetNextPathSquareIndex))) 1) (.collum (Utilities|Array|Get(acopy) _gridarray_5 (Variables|Default|GetNextPathSquareIndex))) (.squaretype (Utilities|Array|Get(acopy) _gridarray_5 (Variables|Default|GetNextPathSquareIndex))) (.visible? (Utilities|Array|Get(acopy) _gridarray_5 (Variables|Default|GetNextPathSquareIndex))) (.squaretyperef (Utilities|Array|Get(acopy) _gridarray_5 (Variables|Default|GetNextPathSquareIndex))))))) (.squaretype (Utilities|Array|Get(acopy) _gridarray_5 (Utilities|Array|FindItem _gridarray_5 (Utilities|Struct|MakeGridSquareStructure (+ (.row (Utilities|Array|Get(acopy) _gridarray_5 (Variables|Default|GetNextPathSquareIndex))) 1) (.collum (Utilities|Array|Get(acopy) _gridarray_5 (Variables|Default|GetNextPathSquareIndex))) (.squaretype (Utilities|Array|Get(acopy) _gridarray_5 (Variables|Default|GetNextPathSquareIndex))) (.visible? (Utilities|Array|Get(acopy) _gridarray_5 (Variables|Default|GetNextPathSquareIndex))) (.squaretyperef (Utilities|Array|Get(acopy) _gridarray_5 (Variables|Default|GetNextPathSquareIndex))))))) (.visible? (Utilities|Array|Get(acopy) _gridarray_5 (Utilities|Array|FindItem _gridarray_5 (Utilities|Struct|MakeGridSquareStructure (+ (.row (Utilities|Array|Get(acopy) _gridarray_5 (Variables|Default|GetNextPathSquareIndex))) 1) (.collum (Utilities|Array|Get(acopy) _gridarray_5 (Variables|Default|GetNextPathSquareIndex))) (.squaretype (Utilities|Array|Get(acopy) _gridarray_5 (Variables|Default|GetNextPathSquareIndex))) (.visible? (Utilities|Array|Get(acopy) _gridarray_5 (Variables|Default|GetNextPathSquareIndex))) (.squaretyperef (Utilities|Array|Get(acopy) _gridarray_5 (Variables|Default|GetNextPathSquareIndex))))))) (.squaretyperef (Utilities|Array|Get(acopy) _gridarray_5 (Utilities|Array|FindItem _gridarray_5 (Utilities|Struct|MakeGridSquareStructure (+ (.row (Utilities|Array|Get(acopy) _gridarray_5 (Variables|Default|GetNextPathSquareIndex))) 1) (.collum (Utilities|Array|Get(acopy) _gridarray_5 (Variables|Default|GetNextPathSquareIndex))) (.squaretype (Utilities|Array|Get(acopy) _gridarray_5 (Variables|Default|GetNextPathSquareIndex))) (.visible? (Utilities|Array|Get(acopy) _gridarray_5 (Variables|Default|GetNextPathSquareIndex))) (.squaretyperef (Utilities|Array|Get(acopy) _gridarray_5 (Variables|Default|GetNextPathSquareIndex))))))))))
              (if (and (Utilities|Array|IsValidIndex _gridarray_3 (Utilities|Array|FindItem _gridarray_3 (Utilities|Struct|MakeGridSquareStructure (- (.row (Utilities|Array|Get(acopy) _gridarray_5 (Variables|Default|GetNextPathSquareIndex))) 1) (.collum (Utilities|Array|Get(acopy) _gridarray_5 (Variables|Default|GetNextPathSquareIndex))) (.squaretype (Utilities|Array|Get(acopy) _gridarray_5 (Variables|Default|GetNextPathSquareIndex))) (.visible? (Utilities|Array|Get(acopy) _gridarray_5 (Variables|Default|GetNextPathSquareIndex))) (.squaretyperef (Utilities|Array|Get(acopy) _gridarray_5 (Variables|Default|GetNextPathSquareIndex)))))) (== (.squaretype (Utilities|Array|Get(acopy) _gridarray_3 (Utilities|Array|FindItem _gridarray_3 (Utilities|Struct|MakeGridSquareStructure (- (.row (Utilities|Array|Get(acopy) _gridarray_5 (Variables|Default|GetNextPathSquareIndex))) 1) (.collum (Utilities|Array|Get(acopy) _gridarray_5 (Variables|Default|GetNextPathSquareIndex))) (.squaretype (Utilities|Array|Get(acopy) _gridarray_5 (Variables|Default|GetNextPathSquareIndex))) (.visible? (Utilities|Array|Get(acopy) _gridarray_5 (Variables|Default|GetNextPathSquareIndex))) (.squaretyperef (Utilities|Array|Get(acopy) _gridarray_5 (Variables|Default|GetNextPathSquareIndex))))))) 0))
                (Utilities|Array|Add (Variables|Default|GetTempGridArray) (Utilities|Struct|MakeGridSquareStructure (.row (Utilities|Array|Get(acopy) _gridarray_3 (Utilities|Array|FindItem _gridarray_3 (Utilities|Struct|MakeGridSquareStructure (- (.row (Utilities|Array|Get(acopy) _gridarray_5 (Variables|Default|GetNextPathSquareIndex))) 1) (.collum (Utilities|Array|Get(acopy) _gridarray_5 (Variables|Default|GetNextPathSquareIndex))) (.squaretype (Utilities|Array|Get(acopy) _gridarray_5 (Variables|Default|GetNextPathSquareIndex))) (.visible? (Utilities|Array|Get(acopy) _gridarray_5 (Variables|Default|GetNextPathSquareIndex))) (.squaretyperef (Utilities|Array|Get(acopy) _gridarray_5 (Variables|Default|GetNextPathSquareIndex))))))) (.collum (Utilities|Array|Get(acopy) _gridarray_3 (Utilities|Array|FindItem _gridarray_3 (Utilities|Struct|MakeGridSquareStructure (- (.row (Utilities|Array|Get(acopy) _gridarray_5 (Variables|Default|GetNextPathSquareIndex))) 1) (.collum (Utilities|Array|Get(acopy) _gridarray_5 (Variables|Default|GetNextPathSquareIndex))) (.squaretype (Utilities|Array|Get(acopy) _gridarray_5 (Variables|Default|GetNextPathSquareIndex))) (.visible? (Utilities|Array|Get(acopy) _gridarray_5 (Variables|Default|GetNextPathSquareIndex))) (.squaretyperef (Utilities|Array|Get(acopy) _gridarray_5 (Variables|Default|GetNextPathSquareIndex))))))) (.squaretype (Utilities|Array|Get(acopy) _gridarray_3 (Utilities|Array|FindItem _gridarray_3 (Utilities|Struct|MakeGridSquareStructure (- (.row (Utilities|Array|Get(acopy) _gridarray_5 (Variables|Default|GetNextPathSquareIndex))) 1) (.collum (Utilities|Array|Get(acopy) _gridarray_5 (Variables|Default|GetNextPathSquareIndex))) (.squaretype (Utilities|Array|Get(acopy) _gridarray_5 (Variables|Default|GetNextPathSquareIndex))) (.visible? (Utilities|Array|Get(acopy) _gridarray_5 (Variables|Default|GetNextPathSquareIndex))) (.squaretyperef (Utilities|Array|Get(acopy) _gridarray_5 (Variables|Default|GetNextPathSquareIndex))))))) (.visible? (Utilities|Array|Get(acopy) _gridarray_3 (Utilities|Array|FindItem _gridarray_3 (Utilities|Struct|MakeGridSquareStructure (- (.row (Utilities|Array|Get(acopy) _gridarray_5 (Variables|Default|GetNextPathSquareIndex))) 1) (.collum (Utilities|Array|Get(acopy) _gridarray_5 (Variables|Default|GetNextPathSquareIndex))) (.squaretype (Utilities|Array|Get(acopy) _gridarray_5 (Variables|Default|GetNextPathSquareIndex))) (.visible? (Utilities|Array|Get(acopy) _gridarray_5 (Variables|Default|GetNextPathSquareIndex))) (.squaretyperef (Utilities|Array|Get(acopy) _gridarray_5 (Variables|Default|GetNextPathSquareIndex))))))) (.squaretyperef (Utilities|Array|Get(acopy) _gridarray_3 (Utilities|Array|FindItem _gridarray_3 (Utilities|Struct|MakeGridSquareStructure (- (.row (Utilities|Array|Get(acopy) _gridarray_5 (Variables|Default|GetNextPathSquareIndex))) 1) (.collum (Utilities|Array|Get(acopy) _gridarray_5 (Variables|Default|GetNextPathSquareIndex))) (.squaretype (Utilities|Array|Get(acopy) _gridarray_5 (Variables|Default|GetNextPathSquareIndex))) (.visible? (Utilities|Array|Get(acopy) _gridarray_5 (Variables|Default|GetNextPathSquareIndex))) (.squaretyperef (Utilities|Array|Get(acopy) _gridarray_5 (Variables|Default|GetNextPathSquareIndex)))))))))))
            (:then_2
              (if (== (Utilities|Array|Length (Variables|Default|GetTempGridArray)) 0)
                (Development|PrintString "braske")
                (goto _label Break)
                (else
                  (bind _output_get_2 (Variables|Default|SetTempSquareType (Math|Random|RandomIntegerinRange 1 2)))
                  (bind _output_get_3 (Variables|Default|SetTempIndex (Math|Random|RandomIntegerinRange 0 (- (Utilities|Array|Length _tempgridarray) 1))))
                  (bind _output_get_4 (Variables|Default|SetNextPathSquareIndex (Utilities|Array|FindItem _gridarray_4 (Utilities|Struct|MakeGridSquareStructure (.row (Utilities|Array|Get(acopy) _tempgridarray _output_get_3)) (.collum (Utilities|Array|Get(acopy) _tempgridarray _output_get_3)) (.squaretype (Utilities|Array|Get(acopy) _tempgridarray _output_get_3)) (.visible? (Utilities|Array|Get(acopy) _tempgridarray _output_get_3)) (.squaretyperef (Utilities|Array|Get(acopy) _tempgridarray _output_get_3))))))
                  (Utilities|Array|SetArrayElem _gridarray_4 _output_get_4 (Utilities|Struct|MakeGridSquareStructure (.row (Utilities|Array|Get(acopy) _gridarray_4 (Utilities|Array|FindItem _gridarray_4 (Utilities|Struct|MakeGridSquareStructure (.row (Utilities|Array|Get(acopy) _tempgridarray _output_get_3)) (.collum (Utilities|Array|Get(acopy) _tempgridarray _output_get_3)) (.squaretype (Utilities|Array|Get(acopy) _tempgridarray _output_get_3)) (.visible? (Utilities|Array|Get(acopy) _tempgridarray _output_get_3)) (.squaretyperef (Utilities|Array|Get(acopy) _tempgridarray _output_get_3)))))) (.collum (Utilities|Array|Get(acopy) _gridarray_4 (Utilities|Array|FindItem _gridarray_4 (Utilities|Struct|MakeGridSquareStructure (.row (Utilities|Array|Get(acopy) _tempgridarray _output_get_3)) (.collum (Utilities|Array|Get(acopy) _tempgridarray _output_get_3)) (.squaretype (Utilities|Array|Get(acopy) _tempgridarray _output_get_3)) (.visible? (Utilities|Array|Get(acopy) _tempgridarray _output_get_3)) (.squaretyperef (Utilities|Array|Get(acopy) _tempgridarray _output_get_3)))))) _output_get_2 (.visible? (Utilities|Array|Get(acopy) _gridarray_4 (Utilities|Array|FindItem _gridarray_4 (Utilities|Struct|MakeGridSquareStructure (.row (Utilities|Array|Get(acopy) _tempgridarray _output_get_3)) (.collum (Utilities|Array|Get(acopy) _tempgridarray _output_get_3)) (.squaretype (Utilities|Array|Get(acopy) _tempgridarray _output_get_3)) (.visible? (Utilities|Array|Get(acopy) _tempgridarray _output_get_3)) (.squaretyperef (Utilities|Array|Get(acopy) _tempgridarray _output_get_3)))))) (.squaretyperef (Utilities|Array|Get(acopy) _gridarray_4 (Utilities|Array|FindItem _gridarray_4 (Utilities|Struct|MakeGridSquareStructure (.row (Utilities|Array|Get(acopy) _tempgridarray _output_get_3)) (.collum (Utilities|Array|Get(acopy) _tempgridarray _output_get_3)) (.squaretype (Utilities|Array|Get(acopy) _tempgridarray _output_get_3)) (.visible? (Utilities|Array|Get(acopy) _tempgridarray _output_get_3)) (.squaretyperef (Utilities|Array|Get(acopy) _tempgridarray _output_get_3))))))))
                  (Utilities|Array|Clear (Variables|Default|GetTempGridArray)))))))))
    (:then_2
      (for (_array_element _array_index) _gridarray_6
        (if (not (or (== (.squaretype _array_element) 1) (== (.squaretype _array_element) 2)))
          (bind _output_get_5 (Variables|Default|SetTempSquareType 3))
          (Utilities|Array|SetArrayElem _gridarray_6 _array_index (Utilities|Struct|MakeGridSquareStructure (.row _array_element) (.collum _array_element) _output_get_5 (.visible? _array_element) (.squaretyperef _array_element))))))))

(fn PathCreation2
  (bind _gridarray (Variables|Default|GetGridArray))
  (bind _gridarray_2 (Variables|Default|GetGridArray))
  (bind _gridarray_3 (Variables|Default|GetGridArray))
  (bind _gridarray_4 (Variables|Default|GetGridArray))
  (bind _gridarray_5 (Variables|Default|GetGridArray))
  (Utilities|FlowControl|Sequence
    (:then_0
      ;[0.15 0.15 0.15 0.5] Sets Starting Square
      (bind _output_get (Variables|Default|SetTempIndex (Math|Random|RandomIntegerinRange 0 (- (Variables|Default|GetGridRowCollumNumber) 1))))
      (bind _output_get_2 (Variables|Default|SetTempSquareType (Math|Random|RandomIntegerinRange 1 2)))
      (Utilities|Array|SetArrayElem _gridarray _output_get (Utilities|Struct|MakeGridSquareStructure (.row (Utilities|Array|Get(acopy) _gridarray _output_get)) (.collum (Utilities|Array|Get(acopy) _gridarray _output_get)) _output_get_2 (.visible? (Utilities|Array|Get(acopy) _gridarray _output_get)) (.squaretyperef (Utilities|Array|Get(acopy) _gridarray _output_get)))))
    (:then_1
      ;[0.15 0.15 0.15 0.5] Need a proper end to the loop (Last Index)
      (Utilities|FlowControl|ForLoopwithBreak 0 10 :!label _label
        (:LoopBody
          (switch int (Math|Random|RandomIntegerinRange 1 3)
            (:Default
              (Development|PrintString "Error" :!label _label_2))
            (:0
              (goto _label_2))
            (:1
              (if (Utilities|Array|IsValidIndex (Variables|Default|GetGridArray) (Utilities|Array|FindItem _gridarray_4 (Utilities|Struct|MakeGridSquareStructure (+ (.row (Utilities|Array|Get(acopy) (Variables|Default|GetGridArray) (Variables|Default|GetTempIndex))) 1) (.collum (Utilities|Array|Get(acopy) (Variables|Default|GetGridArray) (Variables|Default|GetTempIndex))) (.squaretype (Utilities|Array|Get(acopy) (Variables|Default|GetGridArray) (Variables|Default|GetTempIndex))) (.visible? (Utilities|Array|Get(acopy) (Variables|Default|GetGridArray) (Variables|Default|GetTempIndex))) (.squaretyperef (Utilities|Array|Get(acopy) (Variables|Default|GetGridArray) (Variables|Default|GetTempIndex))))))
                (if (== (.squaretype (Utilities|Array|Get(acopy) (Variables|Default|GetGridArray) (Utilities|Array|FindItem _gridarray_4 (Utilities|Struct|MakeGridSquareStructure (+ (.row (Utilities|Array|Get(acopy) (Variables|Default|GetGridArray) (Variables|Default|GetTempIndex))) 1) (.collum (Utilities|Array|Get(acopy) (Variables|Default|GetGridArray) (Variables|Default|GetTempIndex))) (.squaretype (Utilities|Array|Get(acopy) (Variables|Default|GetGridArray) (Variables|Default|GetTempIndex))) (.visible? (Utilities|Array|Get(acopy) (Variables|Default|GetGridArray) (Variables|Default|GetTempIndex))) (.squaretyperef (Utilities|Array|Get(acopy) (Variables|Default|GetGridArray) (Variables|Default|GetTempIndex))))))) 0)
                  (bind _output_get_3 (Variables|Default|SetTempSquareType (Math|Random|RandomIntegerinRange 1 2)))
                  (Utilities|Array|SetArrayElem _gridarray_4 (Utilities|Array|FindItem _gridarray_4 (Utilities|Struct|MakeGridSquareStructure (+ (.row (Utilities|Array|Get(acopy) (Variables|Default|GetGridArray) (Variables|Default|GetTempIndex))) 1) (.collum (Utilities|Array|Get(acopy) (Variables|Default|GetGridArray) (Variables|Default|GetTempIndex))) (.squaretype (Utilities|Array|Get(acopy) (Variables|Default|GetGridArray) (Variables|Default|GetTempIndex))) (.visible? (Utilities|Array|Get(acopy) (Variables|Default|GetGridArray) (Variables|Default|GetTempIndex))) (.squaretyperef (Utilities|Array|Get(acopy) (Variables|Default|GetGridArray) (Variables|Default|GetTempIndex))))) (Utilities|Struct|MakeGridSquareStructure (.row (Utilities|Array|Get(acopy) (Variables|Default|GetGridArray) (Utilities|Array|FindItem _gridarray_4 (Utilities|Struct|MakeGridSquareStructure (+ (.row (Utilities|Array|Get(acopy) (Variables|Default|GetGridArray) (Variables|Default|GetTempIndex))) 1) (.collum (Utilities|Array|Get(acopy) (Variables|Default|GetGridArray) (Variables|Default|GetTempIndex))) (.squaretype (Utilities|Array|Get(acopy) (Variables|Default|GetGridArray) (Variables|Default|GetTempIndex))) (.visible? (Utilities|Array|Get(acopy) (Variables|Default|GetGridArray) (Variables|Default|GetTempIndex))) (.squaretyperef (Utilities|Array|Get(acopy) (Variables|Default|GetGridArray) (Variables|Default|GetTempIndex))))))) (.collum (Utilities|Array|Get(acopy) (Variables|Default|GetGridArray) (Utilities|Array|FindItem _gridarray_4 (Utilities|Struct|MakeGridSquareStructure (+ (.row (Utilities|Array|Get(acopy) (Variables|Default|GetGridArray) (Variables|Default|GetTempIndex))) 1) (.collum (Utilities|Array|Get(acopy) (Variables|Default|GetGridArray) (Variables|Default|GetTempIndex))) (.squaretype (Utilities|Array|Get(acopy) (Variables|Default|GetGridArray) (Variables|Default|GetTempIndex))) (.visible? (Utilities|Array|Get(acopy) (Variables|Default|GetGridArray) (Variables|Default|GetTempIndex))) (.squaretyperef (Utilities|Array|Get(acopy) (Variables|Default|GetGridArray) (Variables|Default|GetTempIndex))))))) _output_get_3 (.visible? (Utilities|Array|Get(acopy) (Variables|Default|GetGridArray) (Utilities|Array|FindItem _gridarray_4 (Utilities|Struct|MakeGridSquareStructure (+ (.row (Utilities|Array|Get(acopy) (Variables|Default|GetGridArray) (Variables|Default|GetTempIndex))) 1) (.collum (Utilities|Array|Get(acopy) (Variables|Default|GetGridArray) (Variables|Default|GetTempIndex))) (.squaretype (Utilities|Array|Get(acopy) (Variables|Default|GetGridArray) (Variables|Default|GetTempIndex))) (.visible? (Utilities|Array|Get(acopy) (Variables|Default|GetGridArray) (Variables|Default|GetTempIndex))) (.squaretyperef (Utilities|Array|Get(acopy) (Variables|Default|GetGridArray) (Variables|Default|GetTempIndex))))))) (.squaretyperef (Utilities|Array|Get(acopy) (Variables|Default|GetGridArray) (Utilities|Array|FindItem _gridarray_4 (Utilities|Struct|MakeGridSquareStructure (+ (.row (Utilities|Array|Get(acopy) (Variables|Default|GetGridArray) (Variables|Default|GetTempIndex))) 1) (.collum (Utilities|Array|Get(acopy) (Variables|Default|GetGridArray) (Variables|Default|GetTempIndex))) (.squaretype (Utilities|Array|Get(acopy) (Variables|Default|GetGridArray) (Variables|Default|GetTempIndex))) (.visible? (Utilities|Array|Get(acopy) (Variables|Default|GetGridArray) (Variables|Default|GetTempIndex))) (.squaretyperef (Utilities|Array|Get(acopy) (Variables|Default|GetGridArray) (Variables|Default|GetTempIndex)))))))))
                  (Variables|Default|SetTempIndex (Utilities|Array|FindItem _gridarray_4 (Utilities|Struct|MakeGridSquareStructure (+ (.row (Utilities|Array|Get(acopy) (Variables|Default|GetGridArray) (Variables|Default|GetTempIndex))) 1) (.collum (Utilities|Array|Get(acopy) (Variables|Default|GetGridArray) (Variables|Default|GetTempIndex))) (.squaretype (Utilities|Array|Get(acopy) (Variables|Default|GetGridArray) (Variables|Default|GetTempIndex))) (.visible? (Utilities|Array|Get(acopy) (Variables|Default|GetGridArray) (Variables|Default|GetTempIndex))) (.squaretyperef (Utilities|Array|Get(acopy) (Variables|Default|GetGridArray) (Variables|Default|GetTempIndex)))))))
                ;[0.15 0.15 0.15 0.5] Still needs to be tested
                (if (Math|Boolean|NANDBoolean (and (Utilities|Array|IsValidIndex (Variables|Default|GetGridArray) (Utilities|Array|FindItem _gridarray_4 (Utilities|Struct|MakeGridSquareStructure (+ (.row (Utilities|Array|Get(acopy) (Variables|Default|GetGridArray) (Variables|Default|GetTempIndex))) 1) (.collum (Utilities|Array|Get(acopy) (Variables|Default|GetGridArray) (Variables|Default|GetTempIndex))) (.squaretype (Utilities|Array|Get(acopy) (Variables|Default|GetGridArray) (Variables|Default|GetTempIndex))) (.visible? (Utilities|Array|Get(acopy) (Variables|Default|GetGridArray) (Variables|Default|GetTempIndex))) (.squaretyperef (Utilities|Array|Get(acopy) (Variables|Default|GetGridArray) (Variables|Default|GetTempIndex)))))) (== (.squaretype (Utilities|Array|Get(acopy) (Variables|Default|GetGridArray) (Utilities|Array|FindItem _gridarray_4 (Utilities|Struct|MakeGridSquareStructure (+ (.row (Utilities|Array|Get(acopy) (Variables|Default|GetGridArray) (Variables|Default|GetTempIndex))) 1) (.collum (Utilities|Array|Get(acopy) (Variables|Default|GetGridArray) (Variables|Default|GetTempIndex))) (.squaretype (Utilities|Array|Get(acopy) (Variables|Default|GetGridArray) (Variables|Default|GetTempIndex))) (.visible? (Utilities|Array|Get(acopy) (Variables|Default|GetGridArray) (Variables|Default|GetTempIndex))) (.squaretyperef (Utilities|Array|Get(acopy) (Variables|Default|GetGridArray) (Variables|Default|GetTempIndex))))))) 0)) (and (Utilities|Array|IsValidIndex (Variables|Default|GetGridArray) (Utilities|Array|FindItem _gridarray_5 (Utilities|Struct|MakeGridSquareStructure (.row (Utilities|Array|Get(acopy) (Variables|Default|GetGridArray) (Variables|Default|GetTempIndex))) (+ (.collum (Utilities|Array|Get(acopy) (Variables|Default|GetGridArray) (Variables|Default|GetTempIndex))) 1) (.squaretype (Utilities|Array|Get(acopy) (Variables|Default|GetGridArray) (Variables|Default|GetTempIndex))) (.visible? (Utilities|Array|Get(acopy) (Variables|Default|GetGridArray) (Variables|Default|GetTempIndex))) (.squaretyperef (Utilities|Array|Get(acopy) (Variables|Default|GetGridArray) (Variables|Default|GetTempIndex)))))) (== (.squaretype (Utilities|Array|Get(acopy) (Variables|Default|GetGridArray) (Utilities|Array|FindItem _gridarray_5 (Utilities|Struct|MakeGridSquareStructure (.row (Utilities|Array|Get(acopy) (Variables|Default|GetGridArray) (Variables|Default|GetTempIndex))) (+ (.collum (Utilities|Array|Get(acopy) (Variables|Default|GetGridArray) (Variables|Default|GetTempIndex))) 1) (.squaretype (Utilities|Array|Get(acopy) (Variables|Default|GetGridArray) (Variables|Default|GetTempIndex))) (.visible? (Utilities|Array|Get(acopy) (Variables|Default|GetGridArray) (Variables|Default|GetTempIndex))) (.squaretyperef (Utilities|Array|Get(acopy) (Variables|Default|GetGridArray) (Variables|Default|GetTempIndex))))))) 0)) (and (Utilities|Array|IsValidIndex (Variables|Default|GetGridArray) (Utilities|Array|FindItem _gridarray_3 (Utilities|Struct|MakeGridSquareStructure (- (.row (Utilities|Array|Get(acopy) (Variables|Default|GetGridArray) (Variables|Default|GetTempIndex))) 1) (.collum (Utilities|Array|Get(acopy) (Variables|Default|GetGridArray) (Variables|Default|GetTempIndex))) (.squaretype (Utilities|Array|Get(acopy) (Variables|Default|GetGridArray) (Variables|Default|GetTempIndex))) (.visible? (Utilities|Array|Get(acopy) (Variables|Default|GetGridArray) (Variables|Default|GetTempIndex))) (.squaretyperef (Utilities|Array|Get(acopy) (Variables|Default|GetGridArray) (Variables|Default|GetTempIndex)))))) (== (.squaretype (Utilities|Array|Get(acopy) (Variables|Default|GetGridArray) (Utilities|Array|FindItem _gridarray_3 (Utilities|Struct|MakeGridSquareStructure (- (.row (Utilities|Array|Get(acopy) (Variables|Default|GetGridArray) (Variables|Default|GetTempIndex))) 1) (.collum (Utilities|Array|Get(acopy) (Variables|Default|GetGridArray) (Variables|Default|GetTempIndex))) (.squaretype (Utilities|Array|Get(acopy) (Variables|Default|GetGridArray) (Variables|Default|GetTempIndex))) (.visible? (Utilities|Array|Get(acopy) (Variables|Default|GetGridArray) (Variables|Default|GetTempIndex))) (.squaretyperef (Utilities|Array|Get(acopy) (Variables|Default|GetGridArray) (Variables|Default|GetTempIndex))))))) 0))) :!label _label_3
                  (goto _label Break))))
            (:2
              (if (Utilities|Array|IsValidIndex (Variables|Default|GetGridArray) (Utilities|Array|FindItem _gridarray_5 (Utilities|Struct|MakeGridSquareStructure (.row (Utilities|Array|Get(acopy) (Variables|Default|GetGridArray) (Variables|Default|GetTempIndex))) (+ (.collum (Utilities|Array|Get(acopy) (Variables|Default|GetGridArray) (Variables|Default|GetTempIndex))) 1) (.squaretype (Utilities|Array|Get(acopy) (Variables|Default|GetGridArray) (Variables|Default|GetTempIndex))) (.visible? (Utilities|Array|Get(acopy) (Variables|Default|GetGridArray) (Variables|Default|GetTempIndex))) (.squaretyperef (Utilities|Array|Get(acopy) (Variables|Default|GetGridArray) (Variables|Default|GetTempIndex))))))
                (if (== (.squaretype (Utilities|Array|Get(acopy) (Variables|Default|GetGridArray) (Utilities|Array|FindItem _gridarray_5 (Utilities|Struct|MakeGridSquareStructure (.row (Utilities|Array|Get(acopy) (Variables|Default|GetGridArray) (Variables|Default|GetTempIndex))) (+ (.collum (Utilities|Array|Get(acopy) (Variables|Default|GetGridArray) (Variables|Default|GetTempIndex))) 1) (.squaretype (Utilities|Array|Get(acopy) (Variables|Default|GetGridArray) (Variables|Default|GetTempIndex))) (.visible? (Utilities|Array|Get(acopy) (Variables|Default|GetGridArray) (Variables|Default|GetTempIndex))) (.squaretyperef (Utilities|Array|Get(acopy) (Variables|Default|GetGridArray) (Variables|Default|GetTempIndex))))))) 0)
                  (bind _output_get_4 (Variables|Default|SetTempSquareType (Math|Random|RandomIntegerinRange 1 2)))
                  (Utilities|Array|SetArrayElem _gridarray_5 (Utilities|Array|FindItem _gridarray_5 (Utilities|Struct|MakeGridSquareStructure (.row (Utilities|Array|Get(acopy) (Variables|Default|GetGridArray) (Variables|Default|GetTempIndex))) (+ (.collum (Utilities|Array|Get(acopy) (Variables|Default|GetGridArray) (Variables|Default|GetTempIndex))) 1) (.squaretype (Utilities|Array|Get(acopy) (Variables|Default|GetGridArray) (Variables|Default|GetTempIndex))) (.visible? (Utilities|Array|Get(acopy) (Variables|Default|GetGridArray) (Variables|Default|GetTempIndex))) (.squaretyperef (Utilities|Array|Get(acopy) (Variables|Default|GetGridArray) (Variables|Default|GetTempIndex))))) (Utilities|Struct|MakeGridSquareStructure (.row (Utilities|Array|Get(acopy) (Variables|Default|GetGridArray) (Utilities|Array|FindItem _gridarray_5 (Utilities|Struct|MakeGridSquareStructure (.row (Utilities|Array|Get(acopy) (Variables|Default|GetGridArray) (Variables|Default|GetTempIndex))) (+ (.collum (Utilities|Array|Get(acopy) (Variables|Default|GetGridArray) (Variables|Default|GetTempIndex))) 1) (.squaretype (Utilities|Array|Get(acopy) (Variables|Default|GetGridArray) (Variables|Default|GetTempIndex))) (.visible? (Utilities|Array|Get(acopy) (Variables|Default|GetGridArray) (Variables|Default|GetTempIndex))) (.squaretyperef (Utilities|Array|Get(acopy) (Variables|Default|GetGridArray) (Variables|Default|GetTempIndex))))))) (.collum (Utilities|Array|Get(acopy) (Variables|Default|GetGridArray) (Utilities|Array|FindItem _gridarray_5 (Utilities|Struct|MakeGridSquareStructure (.row (Utilities|Array|Get(acopy) (Variables|Default|GetGridArray) (Variables|Default|GetTempIndex))) (+ (.collum (Utilities|Array|Get(acopy) (Variables|Default|GetGridArray) (Variables|Default|GetTempIndex))) 1) (.squaretype (Utilities|Array|Get(acopy) (Variables|Default|GetGridArray) (Variables|Default|GetTempIndex))) (.visible? (Utilities|Array|Get(acopy) (Variables|Default|GetGridArray) (Variables|Default|GetTempIndex))) (.squaretyperef (Utilities|Array|Get(acopy) (Variables|Default|GetGridArray) (Variables|Default|GetTempIndex))))))) _output_get_4 (.visible? (Utilities|Array|Get(acopy) (Variables|Default|GetGridArray) (Utilities|Array|FindItem _gridarray_5 (Utilities|Struct|MakeGridSquareStructure (.row (Utilities|Array|Get(acopy) (Variables|Default|GetGridArray) (Variables|Default|GetTempIndex))) (+ (.collum (Utilities|Array|Get(acopy) (Variables|Default|GetGridArray) (Variables|Default|GetTempIndex))) 1) (.squaretype (Utilities|Array|Get(acopy) (Variables|Default|GetGridArray) (Variables|Default|GetTempIndex))) (.visible? (Utilities|Array|Get(acopy) (Variables|Default|GetGridArray) (Variables|Default|GetTempIndex))) (.squaretyperef (Utilities|Array|Get(acopy) (Variables|Default|GetGridArray) (Variables|Default|GetTempIndex))))))) (.squaretyperef (Utilities|Array|Get(acopy) (Variables|Default|GetGridArray) (Utilities|Array|FindItem _gridarray_5 (Utilities|Struct|MakeGridSquareStructure (.row (Utilities|Array|Get(acopy) (Variables|Default|GetGridArray) (Variables|Default|GetTempIndex))) (+ (.collum (Utilities|Array|Get(acopy) (Variables|Default|GetGridArray) (Variables|Default|GetTempIndex))) 1) (.squaretype (Utilities|Array|Get(acopy) (Variables|Default|GetGridArray) (Variables|Default|GetTempIndex))) (.visible? (Utilities|Array|Get(acopy) (Variables|Default|GetGridArray) (Variables|Default|GetTempIndex))) (.squaretyperef (Utilities|Array|Get(acopy) (Variables|Default|GetGridArray) (Variables|Default|GetTempIndex)))))))))
                  (Variables|Default|SetTempIndex (Utilities|Array|FindItem _gridarray_5 (Utilities|Struct|MakeGridSquareStructure (.row (Utilities|Array|Get(acopy) (Variables|Default|GetGridArray) (Variables|Default|GetTempIndex))) (+ (.collum (Utilities|Array|Get(acopy) (Variables|Default|GetGridArray) (Variables|Default|GetTempIndex))) 1) (.squaretype (Utilities|Array|Get(acopy) (Variables|Default|GetGridArray) (Variables|Default|GetTempIndex))) (.visible? (Utilities|Array|Get(acopy) (Variables|Default|GetGridArray) (Variables|Default|GetTempIndex))) (.squaretyperef (Utilities|Array|Get(acopy) (Variables|Default|GetGridArray) (Variables|Default|GetTempIndex))))))
                  (goto _label_3)
                  (else
                    (goto _label_3)))))
            (:3
              (if (Utilities|Array|IsValidIndex (Variables|Default|GetGridArray) (Utilities|Array|FindItem _gridarray_3 (Utilities|Struct|MakeGridSquareStructure (- (.row (Utilities|Array|Get(acopy) (Variables|Default|GetGridArray) (Variables|Default|GetTempIndex))) 1) (.collum (Utilities|Array|Get(acopy) (Variables|Default|GetGridArray) (Variables|Default|GetTempIndex))) (.squaretype (Utilities|Array|Get(acopy) (Variables|Default|GetGridArray) (Variables|Default|GetTempIndex))) (.visible? (Utilities|Array|Get(acopy) (Variables|Default|GetGridArray) (Variables|Default|GetTempIndex))) (.squaretyperef (Utilities|Array|Get(acopy) (Variables|Default|GetGridArray) (Variables|Default|GetTempIndex))))))
                (if (== (.squaretype (Utilities|Array|Get(acopy) (Variables|Default|GetGridArray) (Utilities|Array|FindItem _gridarray_3 (Utilities|Struct|MakeGridSquareStructure (- (.row (Utilities|Array|Get(acopy) (Variables|Default|GetGridArray) (Variables|Default|GetTempIndex))) 1) (.collum (Utilities|Array|Get(acopy) (Variables|Default|GetGridArray) (Variables|Default|GetTempIndex))) (.squaretype (Utilities|Array|Get(acopy) (Variables|Default|GetGridArray) (Variables|Default|GetTempIndex))) (.visible? (Utilities|Array|Get(acopy) (Variables|Default|GetGridArray) (Variables|Default|GetTempIndex))) (.squaretyperef (Utilities|Array|Get(acopy) (Variables|Default|GetGridArray) (Variables|Default|GetTempIndex))))))) 0)
                  (bind _output_get_5 (Variables|Default|SetTempSquareType (Math|Random|RandomIntegerinRange 1 2)))
                  (Utilities|Array|SetArrayElem _gridarray_3 (Utilities|Array|FindItem _gridarray_3 (Utilities|Struct|MakeGridSquareStructure (- (.row (Utilities|Array|Get(acopy) (Variables|Default|GetGridArray) (Variables|Default|GetTempIndex))) 1) (.collum (Utilities|Array|Get(acopy) (Variables|Default|GetGridArray) (Variables|Default|GetTempIndex))) (.squaretype (Utilities|Array|Get(acopy) (Variables|Default|GetGridArray) (Variables|Default|GetTempIndex))) (.visible? (Utilities|Array|Get(acopy) (Variables|Default|GetGridArray) (Variables|Default|GetTempIndex))) (.squaretyperef (Utilities|Array|Get(acopy) (Variables|Default|GetGridArray) (Variables|Default|GetTempIndex))))) (Utilities|Struct|MakeGridSquareStructure (.row (Utilities|Array|Get(acopy) (Variables|Default|GetGridArray) (Utilities|Array|FindItem _gridarray_3 (Utilities|Struct|MakeGridSquareStructure (- (.row (Utilities|Array|Get(acopy) (Variables|Default|GetGridArray) (Variables|Default|GetTempIndex))) 1) (.collum (Utilities|Array|Get(acopy) (Variables|Default|GetGridArray) (Variables|Default|GetTempIndex))) (.squaretype (Utilities|Array|Get(acopy) (Variables|Default|GetGridArray) (Variables|Default|GetTempIndex))) (.visible? (Utilities|Array|Get(acopy) (Variables|Default|GetGridArray) (Variables|Default|GetTempIndex))) (.squaretyperef (Utilities|Array|Get(acopy) (Variables|Default|GetGridArray) (Variables|Default|GetTempIndex))))))) (.collum (Utilities|Array|Get(acopy) (Variables|Default|GetGridArray) (Utilities|Array|FindItem _gridarray_3 (Utilities|Struct|MakeGridSquareStructure (- (.row (Utilities|Array|Get(acopy) (Variables|Default|GetGridArray) (Variables|Default|GetTempIndex))) 1) (.collum (Utilities|Array|Get(acopy) (Variables|Default|GetGridArray) (Variables|Default|GetTempIndex))) (.squaretype (Utilities|Array|Get(acopy) (Variables|Default|GetGridArray) (Variables|Default|GetTempIndex))) (.visible? (Utilities|Array|Get(acopy) (Variables|Default|GetGridArray) (Variables|Default|GetTempIndex))) (.squaretyperef (Utilities|Array|Get(acopy) (Variables|Default|GetGridArray) (Variables|Default|GetTempIndex))))))) _output_get_5 (.visible? (Utilities|Array|Get(acopy) (Variables|Default|GetGridArray) (Utilities|Array|FindItem _gridarray_3 (Utilities|Struct|MakeGridSquareStructure (- (.row (Utilities|Array|Get(acopy) (Variables|Default|GetGridArray) (Variables|Default|GetTempIndex))) 1) (.collum (Utilities|Array|Get(acopy) (Variables|Default|GetGridArray) (Variables|Default|GetTempIndex))) (.squaretype (Utilities|Array|Get(acopy) (Variables|Default|GetGridArray) (Variables|Default|GetTempIndex))) (.visible? (Utilities|Array|Get(acopy) (Variables|Default|GetGridArray) (Variables|Default|GetTempIndex))) (.squaretyperef (Utilities|Array|Get(acopy) (Variables|Default|GetGridArray) (Variables|Default|GetTempIndex))))))) (.squaretyperef (Utilities|Array|Get(acopy) (Variables|Default|GetGridArray) (Utilities|Array|FindItem _gridarray_3 (Utilities|Struct|MakeGridSquareStructure (- (.row (Utilities|Array|Get(acopy) (Variables|Default|GetGridArray) (Variables|Default|GetTempIndex))) 1) (.collum (Utilities|Array|Get(acopy) (Variables|Default|GetGridArray) (Variables|Default|GetTempIndex))) (.squaretype (Utilities|Array|Get(acopy) (Variables|Default|GetGridArray) (Variables|Default|GetTempIndex))) (.visible? (Utilities|Array|Get(acopy) (Variables|Default|GetGridArray) (Variables|Default|GetTempIndex))) (.squaretyperef (Utilities|Array|Get(acopy) (Variables|Default|GetGridArray) (Variables|Default|GetTempIndex)))))))))
                  (Variables|Default|SetTempIndex (Utilities|Array|FindItem _gridarray_3 (Utilities|Struct|MakeGridSquareStructure (- (.row (Utilities|Array|Get(acopy) (Variables|Default|GetGridArray) (Variables|Default|GetTempIndex))) 1) (.collum (Utilities|Array|Get(acopy) (Variables|Default|GetGridArray) (Variables|Default|GetTempIndex))) (.squaretype (Utilities|Array|Get(acopy) (Variables|Default|GetGridArray) (Variables|Default|GetTempIndex))) (.visible? (Utilities|Array|Get(acopy) (Variables|Default|GetGridArray) (Variables|Default|GetTempIndex))) (.squaretyperef (Utilities|Array|Get(acopy) (Variables|Default|GetGridArray) (Variables|Default|GetTempIndex))))))
                  (goto _label_3)
                  (else
                    (goto _label_3)))))))
        (:Completed
          (Development|PrintString "Hello"))))
    (:then_2
      (for (_array_element _array_index) _gridarray_2
        (if (not (or (== (.squaretype _array_element) 1) (== (.squaretype _array_element) 2)))
          (bind _output_get_6 (Variables|Default|SetTempSquareType 3))
          (Utilities|Array|SetArrayElem _gridarray_2 _array_index (Utilities|Struct|MakeGridSquareStructure (.row _array_element) (.collum _array_element) _output_get_6 (.visible? _array_element) (.squaretyperef _array_element))))))))