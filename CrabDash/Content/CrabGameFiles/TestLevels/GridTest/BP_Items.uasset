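; BP_Items is an item actor in the GridTest level that detects when the BP_GridCrab player stands within its Box collision.
; Box begin and end overlap events cast the other actor to BP_GridCrab and toggle the IsOverlappedByPlayer flag, guarded against repeat triggers.
; Each change only prints debug text; no pickup or other item behavior is implemented.
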(event OnComponentBeginOverlap(Box)
  (params (OverlappedComponent :type Primitive%20Component%20Object%20Reference) (OtherActor :type Actor%20Object%20Reference) (OtherComp :type Primitive%20Component%20Object%20Reference) (OtherBodyIndex :type Integer) (bFromSweep :type Boolean) (SweepResult :type Hit%20Result%20Structure%20%28by%20ref%29))
  (Utilities|Casting|CastToBP_GridCrab OtherActor)
  (if (not (Variables|Default|GetisOverlappedByPlayer))
    (bind _output_get (Variables|Default|SetisOverlappedByPlayer true))
    (Development|PrintString (Utilities|String|ToString(Boolean) _output_get))
    (Development|PrintString "Hello")))

(event OnComponentEndOverlap(Box)
  (params (OverlappedComponent :type Primitive%20Component%20Object%20Reference) (OtherActor :type Actor%20Object%20Reference) (OtherComp :type Primitive%20Component%20Object%20Reference) (OtherBodyIndex :type Integer))
  (Utilities|Casting|CastToBP_GridCrab OtherActor)
  (if (Variables|Default|GetisOverlappedByPlayer)
    (bind _output_get (Variables|Default|SetisOverlappedByPlayer false))
    (Development|PrintString (Utilities|String|ToString(Boolean) _output_get) true true "(R=0.160950,G=1.000000,B=0.169309,A=1.000000)")))

(event EventBeginPlay)

(event Collision|EventActorBeginOverlap
  (params (OtherActor :type Actor%20Object%20Reference)))

(event EventTick
  (params (DeltaSeconds :type Float%20%28single-precision%29)))

(fn ConstructionScript)