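; GM_Grid, likely a game mode for a grid test level, randomly places food, hazard and empty items and later hides them.
; SpawnItems clears Interface_Reveal actors, fills TargetPoints by food and hazard rates, and records start locations; its EventGraph call is unconnected.
; While hiding is flagged active, Tick runs HideItems, interpolating items down by a Z offset.
; Completion checks only the last item's exact height.
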(event EventBeginPlay)

(event EventTick
  (params (DeltaSeconds :type Float%20%28single-precision%29))
  (if (Variables|Default|GetItemsCanHide)
    (if (not (Variables|Default|GetisHideItemsComplete))
      (if (Variables|Default|GetisHideItemsActive)
        (CallFunction|HideItems)))))

(fn ConstructionScript)

(fn SpawnItems
  ;[0.15 0.15 0.15 0.5] Spawn items onto the grid.
  (bind _outactors (Actor|GetAllActorswithInterface "/Game/CrabGameFiles/TestLevels/GridTest/Interface_Reveal.Interface_Reveal_C"))
  (for _array_element _outactors
    (Actor|DestroyActor _array_element))
  (Utilities|Array|Clear (Variables|Default|GetAllItemStartLocations))
  (Variables|Default|SetisHideItemsComplete false)
  (Variables|Default|SetisHideItemsActive false)
  (Variables|Default|SetItemsCanHide false)
  ;;[0.15 0.15 0.15 0.5] Set item totals
  (bind _outactors_2 (Actor|GetAllActorsOfClass "/Script/Engine.TargetPoint"))
  (bind _output_get (Variables|Default|SetSpawnPoints _outactors_2))
  (bind _output_get_2 (Variables|Default|SetTotalSpawnPoints (Utilities|Array|Length _output_get)))
  (Variables|Default|SetTotalFoodItems (Math|Float|Truncate (* _output_get_2 (Variables|Default|GetFoodRate))))
  (Variables|Default|SetTotalHazardItems (Math|Float|Truncate (* _output_get_2 (Variables|Default|GetHazardRate))))
  (Variables|Default|SetTotalEmptyItems (Utilities|Operators|Subtract (Variables|Default|GetTotalSpawnPoints) (Variables|Default|GetTotalFoodItems) (Variables|Default|GetTotalHazardItems)))
  ;;[0.15 0.15 0.15 0.5] Spawn food items.
  (for _index (range 0 (- (Variables|Default|GetTotalFoodItems) 1))
    (bind _output_get_3 (LocalVariables|SetCurrentSpawnPoint (.OutItem (Utilities|Array|Random (Variables|Default|GetSpawnPoints)))))
    (Game|SpawnActorfromClass "/Game/CrabGameFiles/TestLevels/GridTest/BP_Food.BP_Food_C" (Math|Transform|MakeTransform (Transformation|GetActorLocation _output_get_3)) "AdjustIfPossibleButAlwaysSpawn" "MultiplyWithRoot" 0 0)
    (Utilities|Array|RemoveItem (Variables|Default|GetSpawnPoints) (LocalVariables|GetCurrentSpawnPoint)))
  ;;[0.15 0.15 0.15 0.5] Spawn hazard items
  (for _index_2 (range 0 (- (Variables|Default|GetTotalHazardItems) 1))
    (bind _output_get_4 (LocalVariables|SetCurrentSpawnPoint (.OutItem (Utilities|Array|Random (Variables|Default|GetSpawnPoints)))))
    (Game|SpawnActorfromClass "/Game/CrabGameFiles/TestLevels/GridTest/BP_Hazard.BP_Hazard_C" (Math|Transform|MakeTransform (Transformation|GetActorLocation _output_get_4)) "Undefined" "MultiplyWithRoot" 0 0)
    (Utilities|Array|RemoveItem (Variables|Default|GetSpawnPoints) (LocalVariables|GetCurrentSpawnPoint)))
  ;;[0.15 0.15 0.15 0.5] Spawn empty items
  (for _index_3 (range 0 (- (Variables|Default|GetTotalEmptyItems) 1))
    (bind _output_get_5 (LocalVariables|SetCurrentSpawnPoint (.OutItem (Utilities|Array|Random (Variables|Default|GetSpawnPoints)))))
    (Game|SpawnActorfromClass "/Game/CrabGameFiles/TestLevels/GridTest/BP_Empty.BP_Empty_C" (Math|Transform|MakeTransform (Transformation|GetActorLocation _output_get_5)) "Undefined" "MultiplyWithRoot" 0 0)
    (Utilities|Array|RemoveItem (Variables|Default|GetSpawnPoints) (LocalVariables|GetCurrentSpawnPoint)))
  (bind _outactors_3 (Actor|GetAllActorswithInterface "/Game/CrabGameFiles/TestLevels/GridTest/Interface_Reveal.Interface_Reveal_C"))
  (bind _output_get_6 (Variables|Default|SetAllSpawnedItems _outactors_3))
  (for _array_element_2 _output_get_6
    (Utilities|Array|Add (Variables|Default|GetAllItemStartLocations) (Transformation|GetActorLocation _array_element_2)))
  (Variables|Default|SetItemsCanHide true))

(fn HideItems
  ;[0.15 0.15 0.15 0.5] Hide all revealed items
  (bind _outactors (Actor|GetAllActorswithInterface "/Game/CrabGameFiles/TestLevels/GridTest/Interface_Reveal.Interface_Reveal_C"))
  (for (_array_element _array_index) _outactors
    (bind _output_get (LocalVariables|SetCurrentItem _array_element))
    (Transformation|SetActorLocation _output_get (Math|Interpolation|VInterpTo (Transformation|GetActorLocation _output_get) (Math|Vector|MakeVector (.x (Utilities|Array|Get(acopy) (Variables|Default|GetAllItemStartLocations) _array_index)) (.y (Utilities|Array|Get(acopy) (Variables|Default|GetAllItemStartLocations) _array_index)) (- (.z (Utilities|Array|Get(acopy) (Variables|Default|GetAllItemStartLocations) _array_index)) (Variables|Default|GetHide%20Z%20Offset))) (Utilities|Time|GetWorldDeltaSeconds) (Variables|Default|GetHide%20Speed)) false false))
  (if (== (.z (Transformation|GetActorLocation _output_get)) (- (.z (Utilities|Array|Get(acopy) (Variables|Default|GetAllItemStartLocations) _array_index)) (Variables|Default|GetHide%20Z%20Offset)))
    (Variables|Default|SetisHideItemsComplete true)
    (Variables|Default|SetisHideItemsActive false)
    (Variables|Default|SetItemsCanHide false)
    (Development|PrintString "Hiding complete!!")))